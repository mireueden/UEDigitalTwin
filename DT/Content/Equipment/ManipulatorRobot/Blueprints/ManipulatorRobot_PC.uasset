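; Player controller for manipulator robots, mapping keyboard input to cargo spawning and robot control.
; On BeginPlay it caches every ManipulatorRobot_BP and, inside that same loop, looks up the first BP_CargoSpawner, enabling spawn mode if one is valid.
; SpaceBar spawns cargo in spawn mode, otherwise starts all robots.
; P pauses and R resumes all cached robots.
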(event EventBeginPlay
  (bind _outactors (Actor|GetAllActorsOfClass "/Game/Equipment/ManipulatorRobot/Blueprints/ManipulatorRobot/ManipulatorRobot_BP.ManipulatorRobot_BP_C"))
  (for _index (range 0 (- (Utilities|Array|Length _outactors) 1))
    (Utilities|Array|Add (Variables|Default|GetRobots) (Utilities|Array|Get(acopy) _outactors _index))
    (bind _outactors_2 (Actor|GetAllActorsOfClass "/Game/Equipment/ManipulatorRobot/Blueprints/BP_CargoSpawner.BP_CargoSpawner_C"))
    (Utilities|IsValid (Utilities|Array|Get(acopy) _outactors_2)
      (:Is%20Valid
        (Variables|Default|SetSpawner (Utilities|Array|Get(acopy) _outactors_2))
        (Variables|Default|SetIsSpawnMode true)))))

(event Input|KeyboardEvents|SpaceBar
  (params (Key :type Key%20Structure))
  (bind _robots (Variables|Default|GetRobots))
  (:Pressed
    (if (Variables|Default|GetIsSpawnMode)
      (Default|SpawnCargo (Variables|Default|GetSpawner))
      (else
        (for _index (range 0 (- (Utilities|Array|Length _robots) 1))
          (Default|Start (Utilities|Array|Get(acopy) _robots _index)))))))

(event Input|KeyboardEvents|P
  (params (Key :type Key%20Structure))
  (bind _robots (Variables|Default|GetRobots))
  (:Pressed
    (for _index (range 0 (- (Utilities|Array|Length _robots) 1))
      (Default|Pause (Utilities|Array|Get(acopy) _robots _index)))))

(event Input|KeyboardEvents|R
  (params (Key :type Key%20Structure))
  (bind _robots (Variables|Default|GetRobots))
  (:Pressed
    (for _index (range 0 (- (Utilities|Array|Length _robots) 1))
      (Default|Resume (Utilities|Array|Get(acopy) _robots _index)))))

(fn ConstructionScript)