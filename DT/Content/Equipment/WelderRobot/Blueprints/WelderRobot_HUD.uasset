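; WelderRobot_HUD is a HUD Blueprint that shows the welder robot's keyboard controls on screen.
; On each DrawHUD it computes X and Y ratios from the screen size against a 1280x720 reference.
; It then draws a single white hint line for start, pause and resume keys, with position and text scale adjusted by those ratios.
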(event EventBeginPlay)

(event Collision|EventActorBeginOverlap
  (params (OtherActor :type Actor%20Object%20Reference)))

(event EventDrawHUD
  (params (SizeX :type Integer) (SizeY :type Integer))
  (Utilities|FlowControl|Sequence
    (:then_0
      (Variables|Default|SetHUDXRatio (/ (Math|Conversions|ToFloat(Integer) SizeX) 1.28e+03)))
    (:then_1
      (Variables|Default|SetHUDYRatio (/ (Math|Conversions|ToFloat(Integer) SizeY) 7.2e+02)))
    (:then_2
      (HUD|DrawText "Space - Start Action 
P - Pause 
R - Resume" "(R=1.000000,G=1.000000,B=1.000000,A=1.000000)" (* 1e+01 (Variables|Default|GetHUDXRatio)) (* 2e+01 (Variables|Default|GetHUDYRatio)) "/Engine/EngineFonts/Roboto.Roboto" (* 1.0 (Variables|Default|GetHUDYRatio)) false))))

(event EventTick
  (params (DeltaSeconds :type Float%20%28single-precision%29)))

(fn ConstructionScript)