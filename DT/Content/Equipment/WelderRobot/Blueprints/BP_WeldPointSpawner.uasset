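; BP_WeldPointSpawner feeds a random test weld target to a referenced welder robot through its SpawnWeldPoint event.
; When the robot's state allows it, it clears old points and spawns a BP_WelderTargetPoint with a demo sphere at a random angle, distance and height within the robot's range.
; It then registers the point, initializes the robot and starts it; otherwise it prints that the robot is busy.
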(event Custom|SpawnWeldPoint
  (bind _welderrobot (Variables|Default|GetWelderRobot))
  (bind _welderrobot_2 (Variables|Default|GetWelderRobot))
  (bind (_workradius _skipradius _seglen) (Default|GetRobotRange _welderrobot_2))
  ;[1 1 1] Spawn random Weld point
  (if (Utilities|Enum|Equal(Enum) (Variables|/Game/Equipment/WelderRobot/Blueprints/BP_WelderRobot.BP_WelderRobot_C|Getstate (Variables|Default|GetWelderRobot)) "NewEnumerator0")
    (Development|PrintString "Spawn Weld Point")
    ;;[1 0.009645 0] Call ClearWeldPoint before add new points!
    (Default|ClearWeldPoints (Variables|Default|GetWelderRobot))
    ;;[1 1 1] Spawn Target at random location around the robot. Send ref of spawned Target to Cargo. Update Target bounds
    (bind _returnvalue (Game|SpawnActorfromClass "/Game/Equipment/WelderRobot/Blueprints/BP_WelderTargetPoint.BP_WelderTargetPoint_C" (Math|Transform|MakeTransform (+ (Math|Vector|RotateVector (Math|Vector|MakeVector (Math|Random|RandomFloatinRange (* _skipradius 1.5) _workradius) 0.0 0.0) (Math|Rotator|MakeRotator 0.0 0.0 (Math|Random|RandomFloatinRange -1.8e+02 1.8e+02))) (Transformation|GetActorLocation _welderrobot_2) (Math|Vector|MakeVector 0.0 0.0 (Math|Random|RandomFloatinRange 0.0 (/ _seglen 1.0))))) "Undefined" "OverrideRootScale" 0 0))
    (Default|ShowDemoSphere _returnvalue)
    ;;[1 1 1] Add Weld Point
    (Default|AddWeldPoint _welderrobot _returnvalue)
    ;;[1 0.009645 0] Init Robot. Must be called after all points was added
    (Default|InitWelderRobot _welderrobot)
    (Default|Start _welderrobot)
    (else
      (Development|PrintString "Robot is busy. Can't add Weled Point" true true "(R=1.000000,G=0.922478,B=0.000000,A=1.000000)"))))

(fn ConstructionScript)