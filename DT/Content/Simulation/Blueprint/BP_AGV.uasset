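; BP_AGV is an AI-controlled actor in the simulation that turns to face where it is heading.
; On Tick, while its AI controller reports a Moving status, it takes the direction to the immediate move destination and smoothly interpolates its rotation toward it.
; The rotation is set as a teleport, and the movement requests themselves are issued outside this Blueprint.
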(event EventTick
  (params (DeltaSeconds :type Float%20%28single-precision%29))
  (bind _self self)
  (bind _returnvalue (AI|GetAIController _self))
  (Utilities|IsValid _returnvalue
    (:Is%20Valid
      (if (Utilities|Enum|Equal(Enum) (Class|AIController|GetMoveStatus _returnvalue) "Moving")
        (Transformation|SetActorRotation (Math|Interpolation|RInterpTo (Transformation|GetActorRotation) (Math|Rotator|MakeRotfromX (- (Class|AIController|GetImmediateMoveDestination _returnvalue) (Transformation|GetActorLocation))) DeltaSeconds 5.0) true)))))

(fn ConstructionScript)