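; PCG factory actor that builds a rectangular spline footprint, presumably as input for procedural generation.
; The construction script places four local-space points from the actor origin to the X and Y of GridControlLocation, ignoring Z.
; It zeroes every tangent for sharp corners and straight edges, deferring the spline update until the end.
; The event graph holds no active logic.
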(event EventBeginPlay)

(event Collision|EventActorBeginOverlap
  (params (OtherActor :type Actor%20Object%20Reference)))

(event EventTick
  (params (DeltaSeconds :type Float%20%28single-precision%29)))

(fn ConstructionScript
  (bind _returnvalue (Math|Vector|MakeVector 0.0 0.0 0.0))
  (bind _spline (Variables|Default|GetSpline))
  (bind _gridcontrollocation (Variables|Default|GetGridControlLocation))
  (bind (_x _y) (Math|Vector|BreakVector _gridcontrollocation))
  (Utilities|FlowControl|Sequence
    (:then_0
      (Class|SplineComponent|SetOverrideConstructionScript _spline true)
      (Spline|SetSplinePoints _spline (Utilities|Array|MakeArray (Math|Vector|MakeVector 0.0 0.0 0.0) (Math|Vector|MakeVector _x 0.0 0.0) (Math|Vector|MakeVector _x _y 0.0) (Math|Vector|MakeVector 0.0 _y 0.0)) "Local" false)
      (for _index (range 0 (- (Spline|GetNumberOfSplinePoints _spline) 1))
        (Spline|SetTangentsatSplinePoint _spline _index _returnvalue _returnvalue "Local" false))
      (Spline|UpdateSpline _spline))))