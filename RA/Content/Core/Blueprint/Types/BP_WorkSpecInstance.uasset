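; BP_WorkSpecInstance tracks the remaining work categories for one work spec, as an ordered queue.
; Initialize appends the spec's WorkOrder to RemainWorkList, and HasNextWork reports whether any entries remain.
; GetNextWork returns the front entry and removes it unless CheckOnly is set, allowing a peek.
; Callers are expected to check HasNextWork first, since an empty list still returns TargetWorkCategory without assigning it.
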(fn Initialize
  (Utilities|Array|AppendArray (Variables|Default|GetRemainWorkList) (Utilities|Struct|BreakS_WorkSpec (Variables|Default|GetSpec))))

(fn HasNextWork
  (return (Utilities|Array|IsNotEmpty (Variables|Default|GetRemainWorkList))))

(fn GetNextWork
  (params (bCheckOnly :type Boolean))
  (bind _remainworklist (Variables|Default|GetRemainWorkList))
  (if (Utilities|Array|IsValidIndex _remainworklist)
    (LocalVariables|SetTargetWorkCategory (Utilities|Array|Get(acopy) _remainworklist))
    (Utilities|FlowControl|Sequence
      (:then_0
        (if (not bCheckOnly)
          (Utilities|Array|RemoveIndex (Variables|Default|GetRemainWorkList))))
      (:then_1
        (return (LocalVariables|GetTargetWorkCategory))))
    (else
      (return (LocalVariables|GetTargetWorkCategory)))))