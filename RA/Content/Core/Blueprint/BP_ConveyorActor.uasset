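; Conveyor actor that moves BP_Item actors along its spline components and destroys them on overlapping a GoalTrigger.
; AddItem assigns the closest spline; Tick offsets each item along that spline's direction at MoveSpeed.
; At a spline's end, items snap to its XY, keep their Z, and switch to the next spline from a component-reference map.
; DebugItemMove line-traces at a random spline to spawn a test item.
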(event Custom|OnBeginOverlap_GoalTrigger
  (params (OverlappedActor :type Actor%20Object%20Reference) (OtherActor :type Actor%20Object%20Reference))
  (bind _asbp_item (Utilities|Casting|CastToBP_Item OtherActor))
  (CallFunction|RemoveItem _asbp_item)
  (Actor|DestroyActor _asbp_item))

(event EventTick
  (params (DeltaSeconds :type Float%20%28single-precision%29))
  (CallFunction|MoveItems DeltaSeconds))

(event EventBeginPlay
  (Utilities|FlowControl|Sequence
    (:then_0
      (Variables|Default|SetSplineCompList (Actor|GetComponentsByClass "/Script/Engine.SplineComponent")))
    (:then_1
      (bind _goaltrigger (Variables|Default|GetGoalTrigger)
        (:then
          (Collision|BindEventtoOnActorBeginOverlap _goaltrigger (delegate Custom|OnBeginOverlap_GoalTrigger)))
        (:else)))))

(fn ConstructionScript)

(fn AddItem
  (params (NewItem :type BP%20Item%20Object%20Reference))
  (Utilities|IsValid NewItem
    (:Is%20Valid
      (bind _splinecomp (CallFunction|GetClosestSpline (Transformation|GetActorLocation NewItem)))
      (Utilities|IsValid _splinecomp
        (:Is%20Valid
          (Default|SetTargetSpline NewItem _splinecomp)
          (Utilities|Array|Add (Variables|Internal|GetItemList) NewItem))
        (:Is%20Not%20Valid
          (Development|PrintString "Counld not found closest spline (ConveyorActor::AddItem)" true true "(R=1.000000,G=0.000000,B=0.000000,A=1.000000)"))))
    (:Is%20Not%20Valid
      (Development|PrintString "Invalid Item Reference (ConveyorActor::AddItem)" true true "(R=1.000000,G=0.000000,B=0.000000,A=1.000000)"))))

(fn RemoveItem
  (params (Item :type BP%20Item%20Object%20Reference%20%28by%20ref%29))
  (Utilities|Array|RemoveItem (Variables|Internal|GetItemList) Item))

(fn MoveItems
  (params (DeltaTime :type Float%20%28double-precision%29))
  (for _array_element (Variables|Internal|GetItemList)
    (Utilities|IsValid (Default|GetTargetSpline _array_element)
      (:Is%20Valid
        (bind _output_get (LocalVariables|SetMoveAmount (* (Spline|FindDirectionClosesttoWorldLocation (Default|GetTargetSpline _array_element) (Transformation|GetActorLocation _array_element) "World") (* DeltaTime (Variables|Default|GetMoveSpeed)))))
        (if (>= (CallFunction|GetMoveDistanceRate (Default|GetTargetSpline _array_element) (Transformation|GetActorLocation _array_element)) 1.0)
          (Transformation|SetActorLocation _array_element (+ (* (Transformation|GetActorLocation _array_element) "0.000000,0.000000,1.000000") (* (Spline|GetLocationatTime (Default|GetTargetSpline _array_element) 1.0 "World" false) "1.000000,1.000000,0.000000")) false true)
          (Default|SetTargetSpline _array_element (CallFunction|GetNextSpline (Default|GetTargetSpline _array_element)))
          (else
            (Transformation|AddActorWorldOffset _array_element _output_get false true)))))))

(fn DebugItemMove
  (bind _returnvalue (Math|Vector|MakeVector 0.0 0.0 1e+02))
  (LocalVariables|SetRandomSplineComp (.OutItem (Utilities|Array|Random (Utilities|Array|MakeArray (Variables|Default|GetSpline) (Variables|Default|GetSpline1) (Variables|Default|GetSpline2)))))
  (bind (_outhit _returnvalue_2) (Class|KismetSystemLibrary|LineTraceSinglebyProfile (+ (.Location (Math|Transform|BreakTransform (Spline|GetTransformatTime (LocalVariables|GetRandomSplineComp) 0.0 "World" false false))) _returnvalue) (- (.Location (Math|Transform|BreakTransform (Spline|GetTransformatTime (LocalVariables|GetRandomSplineComp) 0.0 "World" false false))) _returnvalue) "BlockAllDynamic" false 0 "ForDuration" true))
  (if _returnvalue_2
    (Rendering|Debug|DrawDebugSphere (+ (.Location (Collision|BreakHitResult _outhit)) "0.000000,0.000000,55.000000") 1e+02 12 "(R=0.000000,G=1.000000,B=0.179306,A=1.000000)" 1e+01 5.0)
    (Development|PrintString (Utilities|String|ToString(Vector) (+ (.Location (Collision|BreakHitResult _outhit)) "0.000000,0.000000,55.000000")))
    (bind _returnvalue_3 (Game|SpawnActorfromClass "/Game/Core/Blueprint/BP_Item.BP_Item_C" (Math|Transform|MakeTransform (+ (.Location (Collision|BreakHitResult _outhit)) "0.000000,0.000000,55.000000")) "Undefined" "MultiplyWithRoot" 0 0))
    (CallFunction|AddItem _returnvalue_3)
    (Default|SetTargetSpline _returnvalue_3 (LocalVariables|GetRandomSplineComp))))

(fn GetNextSpline
  (params (CheckSpline :type Spline%20Component%20Object%20Reference))
  (return (.AsSpline%20Component (Utilities|Casting|CastToSplineComponent (Class|RALibrary|ResolveBaseComponentReference (.Value (Utilities|Map|Find (Variables|Default|GetSplineCompReferenceMap) (Utilities|Struct|MakeBaseComponentReference (Utilities|String|StringToName (Utilities|GetObjectName CheckSpline))))) (Components|GetOwner CheckSpline))))))

(fn GetMoveDistanceRate
  (params (InSplineComp :type Spline%20Component%20Object%20Reference) (InLocation :type Vector%20%28by%20ref%29))
  (return (/ (Class|SplineComponent|GetDistanceAlongSplineatLocation InSplineComp InLocation "World") (Spline|GetSplineLength InSplineComp))))

(fn GetClosestSpline
  (params (FindLocation :type Vector))
  (LocalVariables|SetMinDistanceSquared (Math|Float|Square 1e+05))
  (for _array_element (Variables|Default|GetSplineCompList)
    (bind _output_get (LocalVariables|SetTempDistanceSquared (Class|KismetMathLibrary|VectorDistanceSquared FindLocation (Spline|FindLocationClosesttoWorldLocation _array_element FindLocation "World"))))
    (if (< _output_get (LocalVariables|GetMinDistanceSquared))
      (LocalVariables|SetFoundSpline _array_element)
      (LocalVariables|SetMinDistanceSquared (LocalVariables|GetTempDistanceSquared))))
  (return (LocalVariables|GetFoundSpline)))