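; Delivery bot that carries out an assigned WorkSpec by visiting stock and work shelf queues, then heading to a cargo queue to idle.
; TryNextStep gets queue slots from the RA manager, and NextStep sets the state and starts AI movement.
; AddMovePoints stacks an L-shaped route, Y leg first.
; MoveComplete advances the state only when the list is empty; no live path there starts the second leg.
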(event Custom|MoveComplete
  (params (RequestID :type AI%20Request%20ID%20Structure) (Result :type EPathFollowingResult%20Enum :default "Success"))
  (if (Utilities|Enum|Equal(Enum) Result "Success")
    (if (Utilities|Array|IsEmpty (Variables|Default|GetMovementList))
      (if (Utilities|Enum|Equal(Enum) (Variables|Default|GetBotState) "NewEnumerator5")
        (Variables|Default|SetBotState "NewEnumerator0")
        (Variables|Internal|SetWorkData 0)
        (else
          (bind _output_get (Variables|Default|SetBotState (Utilities|Enum|ByteToEnumE_DeliveryBotState (+ (stale _output_get) 1))))
          (CallFunction|TryNextStep))))
    (else
      (Development|PrintString (Utilities|String|Append "MoveComplete is Failed : " (Utilities|String|ToString(Byte) Result))))))

(event Custom|MoveToNext
  (bind _movementlist (Variables|Default|GetMovementList))
  (bind _returnvalue (Utilities|Array|LastIndex _movementlist))
  (if (!= _returnvalue -1)
    (Utilities|FlowControl|Sequence
      (:then_0
        (AI|Navigation|MovetoLocation (AI|GetAIController self) (Utilities|Array|Get(acopy) _movementlist _returnvalue) -1.0 true true false true 0))
      (:then_1
        (Utilities|Array|RemoveIndex _movementlist _returnvalue)))))

(event Custom|NextStep
  (params (NextTransform :type Transform) (WorkCategory :type E_RACategory%20Enum :default "NewEnumerator0"))
  (bind _location (Math|Transform|BreakTransform NextTransform))
  (bind (_x _y _z) (Math|Vector|BreakVector _location))
  (switch Utilities|FlowControl|Switch|SwitchonE_RACategory WorkCategory
    (:NewEnumerator1
      (Utilities|FlowControl|Sequence
        (:then_0
          (Variables|Default|SetBotState "NewEnumerator3"))
        (:then_1
          (CallFunction|AddMovePoints _location :!label _label)
          (CallFunction|MovetoNext)
          (Development|PrintText (Utilities|Text|FormatText "(X={X},Y={Y},Z={Z})" (Utilities|Text|ToText(Float) _x "HalfToEven" false false) (Utilities|Text|ToText(Float) _y "HalfToEven" false false) (Utilities|Text|ToText(Float) _z "HalfToEven" false false))))))
    (:NewEnumerator3
      (Utilities|FlowControl|Sequence
        (:then_0
          (Variables|Default|SetBotState "NewEnumerator1"))
        (:then_1
          (goto _label))))
    (:NewEnumerator4
      (Utilities|FlowControl|Sequence
        (:then_0
          (Variables|Default|SetBotState "NewEnumerator5"))
        (:then_1
          (goto _label))))))

(event Custom|TryNextStep
  (switch Utilities|FlowControl|Switch|SwitchonE_DeliveryBotState (Variables|Default|GetBotState)
    (:NewEnumerator0
      _)
    (:NewEnumerator2
      _)
    (:NewEnumerator4
      _))
  (bind _workdata (Variables|Internal|GetWorkData)
    (:then
      (if (Default|HasNextWork _workdata)
        (bind _asbp_bot_queue (Default|GetAvailabeQueuebyCategory (CallFunction|GetRAManagerEx) (Default|GetNextWork _workdata true)))
        (if (.bValid (Default|GetQueueTransformat _asbp_bot_queue (Default|GetNextQueueIndex _asbp_bot_queue)))
          (Default|Enqueue _asbp_bot_queue self)
          (CallFunction|NextStep (.Output (Default|GetQueueTransformat _asbp_bot_queue (Default|GetNextQueueIndex _asbp_bot_queue))) (Default|GetNextWork _workdata false))
          (else
            (Development|PrintString "[TODO] TryNextStep...")))
        (else
          (bind _asbp_bot_queue_2 (Default|GetAvailabeQueuebyCategory (CallFunction|GetRAManagerEx) "NewEnumerator4"))
          (if (.bValid (Default|GetQueueTransformat _asbp_bot_queue_2 (Default|GetNextQueueIndex _asbp_bot_queue_2)))
            (CallFunction|NextStep (.Output (Default|GetQueueTransformat _asbp_bot_queue_2 (Default|GetNextQueueIndex _asbp_bot_queue_2))) "NewEnumerator4")))))
    (:else)))

(event Custom|MoveTo
  (params (Dest :type Vector%20%28by%20ref%29))
  (AI|Navigation|MovetoLocation (AI|GetAIController self) Dest -1.0 true true false true 0))

(event EventBeginPlay)

(event EventPossessed
  (params (NewController :type Controller%20Object%20Reference))
  (bind _asaicontroller (Utilities|Casting|CastToAIController NewController))
  (EventDispatchers|BindEventtoReceiveMoveCompleted _asaicontroller (delegate Custom|MoveComplete)))

(event EventUnpossessed
  (params (OldController :type Controller%20Object%20Reference))
  (bind _asaicontroller (Utilities|Casting|CastToAIController OldController))
  (EventDispatchers|UnbindEventfromReceiveMoveCompleted _asaicontroller (delegate Custom|MoveComplete)))

(fn ConstructionScript)

(fn AssignWork
  (params (WorkSpec :type S%20Work%20Spec%20Structure%20%28by%20ref%29))
  (bind _returnvalue (Game|ConstructObjectfromClass "/Game/Core/Blueprint/Types/BP_WorkSpecInstance.BP_WorkSpecInstance_C" WorkSpec))
  (Variables|Internal|SetWorkData _returnvalue)
  (Default|Initialize _returnvalue)
  (CallFunction|TryNextStep))

(fn DebugMoveto
  (bind _returnvalue (Transformation|GetActorLocation))
  (bind (_x _y _z) (Math|Vector|BreakVector _returnvalue))
  (bind _targetpoint (Variables|Default|GetTargetPoint)
    (:then
      (Utilities|FlowControl|Sequence
        (:then_0
          (Utilities|Array|Add (Variables|Default|GetMovementList) (Math|Vector|MakeVector (.X (Math|Vector|BreakVector (Transformation|GetActorLocation _targetpoint))) (.Y (Math|Vector|BreakVector (Transformation|GetActorLocation _targetpoint))) _z))
          (Utilities|Array|Add (Variables|Default|GetMovementList) (Math|Vector|MakeVector _x (.Y (Math|Vector|BreakVector (Transformation|GetActorLocation _targetpoint))) _z)))
        (:then_1
          (CallFunction|MovetoNext))))
    (:else)))

(fn AddMovePoints
  (params (InVec :type Vector))
  (bind _returnvalue (Transformation|GetActorLocation))
  (bind (_x _y) (Math|Vector|BreakVector InVec))
  (bind (_x_2 _y_2 _z) (Math|Vector|BreakVector _returnvalue))
  (Utilities|Array|Add (Variables|Default|GetMovementList) (Math|Vector|MakeVector _x _y _z))
  (Utilities|Array|Add (Variables|Default|GetMovementList) (Math|Vector|MakeVector _x_2 _y _z)))

(fn GetManageCategory
  (return "NewEnumerator2"))