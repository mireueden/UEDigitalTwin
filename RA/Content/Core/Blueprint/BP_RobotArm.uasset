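; Industrial robot arm actor that picks up a nearby idle BP_Item and places it on a conveyor.
; A sphere trace finds the item, then TryNextStep advances an integer state machine through aim, reach, attach, idle, place, release and return.
; Timelines turn the base and move the RobotTarget transform, with their completion or tick-polling flags triggering the next step.
; The construction script sizes the work-radius material display and caches the idle pose.
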(event Custom|FindItemAndTransport
  (bind _returnvalue (Transformation|GetActorLocation))
  (if (== (Variables|Default|GetRobotState) 0)
    (bind (_outhits _returnvalue_2) (Collision|MultiSphereTraceForObjects _returnvalue (+ _returnvalue "0.000000,0.000000,0.001000") 4e+02 (Utilities|Array|MakeArray "ObjectTypeQuery2") false 0 "ForDuration"))
    (if _returnvalue_2
      (bind _array_element (Utilities|Array|ForEachLoopwithBreak _outhits :!label _label)
        (:LoopBody
          (bind _asbp_item (Utilities|Casting|CastToBP_Item (.HitActor (Collision|BreakHitResult _array_element))))
          (if (Default|IsStateEquals _asbp_item "NewEnumerator0")
            (Variables|Default|SetItem _asbp_item)
            (CallFunction|TryNextStep (Variables|Default|GetRobotState))
            (goto _label Break)))))
    (else
      (Development|PrintString "Already working state..."))))

(event Custom|TryNextStep
  (params (CurrentState :type Integer))
  (bind _robotplacetarget (Variables|Default|GetRobotPlaceTarget))
  (bind _item (Variables|Default|GetItem))
  (bind _item_2 (Variables|Default|GetItem))
  (bind _item_3 (Variables|Default|GetItem))
  (bind _returnvalue (Transformation|GetWorldTransform _robotplacetarget))
  (bind _returnvalue_2 (Default|GetPickupTransform _item_2 "RTS_World"))
  (bind _outtransform (Default|GetPlaceTransform _item _returnvalue))
  (Utilities|FlowControl|Delay 1.0)
  (bind _output_get (Variables|Default|SetRobotState (Math|Integer|Clamp(Integer) (+ CurrentState 1) 0 8)))
  (switch int _output_get
    (:1
      (Default|SetItemState _item_2 "NewEnumerator1")
      (CallFunction|SetLookTransform _returnvalue_2))
    (:2
      (CallFunction|SetTargetTransform _returnvalue_2))
    (:3
      ;[0.15 0.15 0.15 0.5] 집게 잡는 연출이 있을 수 있습니다.
      (Transformation|AttachComponentToComponent (Variables|Default|GetItem) (Variables|Default|GetSkeletalMesh) "Robot1_End" "KeepWorld" "KeepWorld" "KeepWorld" true)
      (CallFunction|TryNextStep (Variables|Default|GetRobotState)))
    (:4
      (CallFunction|GoIdlePose false))
    (:5
      (CallFunction|SetLookTransform _outtransform))
    (:6
      (CallFunction|SetTargetTransform _outtransform))
    (:7
      (Transformation|DetachFromActor _item_3 "KeepWorld" "KeepWorld" "KeepWorld")
      (Default|SetItemState _item_3 "NewEnumerator0")
      (Utilities|FlowControl|Sequence
        (:then_0
          (bind _conveyoractor (CallFunction|GetConveyorActor))
          (Utilities|IsValid _conveyoractor
            (:Is%20Valid
              (Default|AddItem _conveyoractor (Variables|Default|GetItem)))
            (:Is%20Not%20Valid
              (Development|PrintString "Invalid ConveyorActor." true true "(R=1.000000,G=0.000000,B=0.000000,A=1.000000)"))))
        (:then_1
          (CallFunction|TryNextStep (Variables|Default|GetRobotState)))))
    (:8
      (CallFunction|GoIdlePose false))))

(event Custom|SetLookTransform
  (params (Transform :type Transform))
  (bind _returnvalue (Transformation|GetActorLocation))
  (bind _location (Math|Transform|BreakTransform Transform))
  (bind _robotbase (Variables|Default|GetRobotBase))
  (bind _returnvalue_2 (- _location _returnvalue))
  (bind _returnvalue_3 (Math|Rotator|MakeRotfromZ _returnvalue_2))
  (bind _yaw (Math|Rotator|BreakRotator _returnvalue_3))
  (bind _returnvalue_4 (+ _yaw -9e+01))
  (bind _returnvalue_5 (Math|Rotator|MakeRotator 0.0 0.0 _returnvalue_4))
  ;[0.15 0.15 0.15 0.5] Robot1_A
  (Variables|Internal|SetbProcessLook true)
  (Timeline|BaseRotateTimeline PlayFromStart
    (:Update
      (Transformation|SetRelativeRotation _robotbase (Math|Interpolation|RInterpTo (Variables|/Script/Engine.SceneComponent|GetRelativeRotation _robotbase) _returnvalue_5 (Utilities|Time|GetWorldDeltaSeconds) 5.0) false false))
    (:Finished
      (Transformation|SetRelativeRotation _robotbase _returnvalue_5 false false)
      (Variables|Internal|SetbProcessLook false)
      (CallFunction|FinishProcess))))

(event Custom|SetTargetTransform
  (params (Transform :type Transform))
  (bind _robottarget (Variables|Default|GetRobotTarget))
  (bind _armmovetimeline (Variables|Default|GetArmMoveTimeline))
  (Variables|Internal|SetbProcessArmMove true)
  (Components|Timeline|SetPlayRate _armmovetimeline (/ (Components|Timeline|GetTimelineLength _armmovetimeline) (Variables|Default|GetArmMoveTime)))
  (bind _rate (Timeline|ArmMoveTimeline PlayFromStart)
    (:Update
      (Transformation|SetWorldTransform _robottarget (Math|Transform|Lerp(Transform) (Transformation|GetWorldTransform _robottarget) Transform _rate) false true))
    (:Finished
      (Transformation|SetWorldTransform _robottarget Transform false true)
      (Variables|Internal|SetbProcessArmMove false)
      (CallFunction|FinishProcess))))

(event Custom|FinishProcess
  (switch int (Variables|Default|GetRobotState)
    (:1
      (CallFunction|TryNextStep (Variables|Default|GetRobotState) :!label _label))
    (:2
      (goto _label))
    (:4
      (if (Variables|Internal|GetbProcessIdlePose) :!label _label_2
        (Utilities|FlowControl|DelayUntilNextTick)
        (goto _label_2)
        (else
          (goto _label))))
    (:5
      (goto _label))
    (:6
      (goto _label))
    (:8
      (if (Variables|Internal|GetbProcessIdlePose) :!label _label_3
        (Utilities|FlowControl|DelayUntilNextTick)
        (goto _label_3)
        (else
          (Variables|Default|SetRobotState 0))))))

(event Custom|GoIdlePose
  (params (bImmediately :type Boolean))
  (bind _targetidletransform (Variables|Internal|GetTargetIdleTransform))
  (if bImmediately
    (Transformation|SetWorldTransform (Variables|Default|GetRobotTarget) _targetidletransform false true)
    (else
      (Variables|Internal|SetbProcessIdlePose true)
      (CallFunction|SetTargetTransform _targetidletransform)
      (if (Variables|Internal|GetbProcessArmMove) :!label _label
        (Utilities|FlowControl|DelayUntilNextTick)
        (goto _label)
        (else
          (Utilities|FlowControl|Delay 0.3)
          (CallFunction|SetLookTransform _targetidletransform)
          (Variables|Internal|SetbProcessIdlePose false))))))

(fn ConstructionScript
  (bind _max (CallFunction|GetWorkRadius))
  (bind (_min _max_2) (CallFunction|GetWorkRadius))
  (bind _plane_workradius (Variables|Default|GetPlane_WorkRadius))
  (bind _returnvalue (* _max 0.01 2.0))
  (Utilities|FlowControl|Sequence
    (:then_0
      (Transformation|SetRelativeScale3D _plane_workradius (Math|Vector|MakeVector _returnvalue _returnvalue 1.0))
      (bind _returnvalue_2 (Rendering|Material|CreateDynamicMaterialInstance _plane_workradius 0 (Rendering|Material|GetMaterial _plane_workradius 0) "None" :!class /Script/Engine.PrimitiveComponent))
      (Rendering|Material|SetMaterial _plane_workradius 0 _returnvalue_2)
      (Rendering|Material|SetScalarParameterValue _returnvalue_2 "OuterRadius" _max_2 :!class /Script/Engine.MaterialInstanceDynamic)
      (Rendering|Material|SetScalarParameterValue _returnvalue_2 "InnerRadius" _min :!class /Script/Engine.MaterialInstanceDynamic))
    (:then_1
      (Variables|Internal|SetTargetIdleTransform (Transformation|GetWorldTransform (Variables|Default|GetRobotTarget))))))

(fn GetControlInitialTransform
  (params (Name :type Name))
  (bind _returnvalue (Class|ControlRig|FindControlRigs self "/Game/Core/Mesh/RobotArm/CR_IndustrialRobot.CR_IndustrialRobot_C"))
  (if (Utilities|Array|IsValidIndex _returnvalue)
    (bind _ascr_industrial_robot (Utilities|Casting|CastToCR_IndustrialRobot (Utilities|Array|Get(acopy) _returnvalue))
      (:then
        (bind _returnvalue_2 (Class|RigHierarchy|GetTransformfromControlValue (Class|RigHierarchy|GetControlValue (Class|ControlRig|GetHierarchy _ascr_industrial_robot) (Utilities|Struct|MakeRigElementKey "Control" Name) "Initial")))
        (return true _returnvalue_2))
      (:CastFailed
        _)))
  (return false ""))

(fn GetWorkRadius
  (bind _workradius (Variables|Default|GetWorkRadius))
  (bind (_lowerbound _upperbound) (Utilities|Struct|BreakFloatRange _workradius))
  (return (.Value (Utilities|Struct|BreakFloatRangeBound _lowerbound)) (.Value (Utilities|Struct|BreakFloatRangeBound _upperbound))))

(fn GetRobotControlRigTransform
  (params (Name :type Name) (Space :type EControlRigComponentSpace%20Enum :default "WorldSpace") (bInitial :type Boolean))
  (bind _returnvalue (Class|ControlRig|FindControlRigs self "/Game/Core/Mesh/RobotArm/CR_IndustrialRobot.CR_IndustrialRobot_C"))
  (if (Utilities|Array|IsValidIndex _returnvalue)
    (return (Class|RAAnimationLibrary|GetControlTransform (Utilities|Array|Get(acopy) _returnvalue) (Variables|Default|GetSkeletalMesh) Name Space bInitial))
    (else
      (return (Math|Transform|MakeTransform "0, 0, 0")))))

(fn GetManageCategory
  (return "NewEnumerator0"))