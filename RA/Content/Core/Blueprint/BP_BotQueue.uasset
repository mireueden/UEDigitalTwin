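; BP_BotQueue is a placeable queue actor that holds bots in line at evenly spaced slots.
; The construction script stretches the box by Capacity, caches centered slot transforms along local X and shows them as debug instanced meshes.
; Bots are stored first-in, first-out; Dequeue removes the front bot and calls AlignBots to walk the rest forward with MoveTo.
; ExecAlignBots teleports them instead, and Enqueue leaves capacity checks to callers via IsQueueFull.
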(event EventBeginPlay)

(fn ConstructionScript
  (bind _ism_debugplace (Variables|Default|GetISM_DebugPlace))
  (bind _box (Variables|Default|GetBox))
  (bind _boxextent (Variables|/Script/Engine.BoxComponent|GetBoxExtent _box))
  (bind _x (Math|Vector|BreakVector _boxextent))
  (bind _output_get (Variables|Default|SetCapacity (Math|Integer|Max(Integer) (Variables|Default|GetCapacity) 1)))
  (Transformation|SetRelativeScale3D (Variables|Default|GetBox) (Math|Vector|MakeVector (Math|Conversions|ToFloat(Integer) _output_get) 1.0 1.0))
  (Utilities|FlowControl|Sequence
    (:then_0
      (Components|InstancedStaticMesh|ClearInstances _ism_debugplace))
    (:then_1
      (for _index (range 0 (- (Variables|Default|GetCapacity) 1))
        (Components|InstancedStaticMesh|AddInstance _ism_debugplace (Math|Transform|MakeTransform (Math|Vector|MakeVector (- (* _x 2.0 _index) (* _x (- (Variables|Default|GetCapacity) 1))) 0.0 0.0)) false)
        (Utilities|Array|Add (Variables|Default|GetTransformList) (Math|Transform|MakeTransform (Math|Vector|MakeVector (- (* _x 2.0 _index) (* _x (- (Variables|Default|GetCapacity) 1))) 0.0 0.0)))))))

(fn Enqueue
  (params (NewItem :type BP%20Delivery%20Bot%20Object%20Reference%20%28by%20ref%29))
  (Utilities|Array|Add (Variables|Default|GetBotList) NewItem))

(fn Dequeue
  (bind _botlist (Variables|Default|GetBotList))
  (Utilities|FlowControl|Sequence
    (:then_0
      (if (Utilities|Array|IsValidIndex _botlist)
        (LocalVariables|SetFoundBot (Utilities|Array|Get(acopy) _botlist))
        (Utilities|Array|RemoveIndex _botlist)))
    (:then_1
      ;[0.15 0.15 0.15 0.5] Check: FoundBot이 해당 위치에서 빠져나간 상태일 때 호출되도록 설정 필요
      (CallFunction|AlignBots))
    (:then_2
      (return (LocalVariables|GetFoundBot)))))

(fn Top
  (bind _botlist (Variables|Default|GetBotList))
  (if (Utilities|Array|IsValidIndex _botlist)
    (return (Utilities|Array|Get(acopy) _botlist))))

(fn IsQueueEmpty
  (return (Utilities|Array|IsEmpty (Variables|Default|GetBotList))))

(fn IsQueueFull
  (return (>= (Utilities|Array|Length (Variables|Default|GetBotList)) (Variables|Default|GetCapacity))))

(fn GetNextQueueIndex
  (return (+ (Utilities|Array|LastIndex (Variables|Default|GetBotList)) 1)))

(fn GetQueueTransformat
  (params (Index :type Integer))
  (bind _transformlist (Variables|Default|GetTransformList))
  (if (Utilities|Array|IsValidIndex _transformlist Index)
    (return (Math|Transform|ComposeTransforms (Utilities|Array|Get(acopy) _transformlist Index) (Transformation|GetActorTransform)) true)
    (else
      (return (Math|Transform|MakeTransform "0, 0, 0") false))))

(fn ExecAlignBots
  (for (_array_element _array_index) (Variables|Default|GetBotList)
    (Transformation|SetActorTransform _array_element (Math|Transform|ComposeTransforms (Utilities|Array|Get(acopy) (Variables|Default|GetTransformList) _array_index) (Transformation|GetActorTransform)) false true)))

(fn AlignBots
  (for (_array_element _array_index) (Variables|Default|GetBotList)
    (Default|Moveto _array_element (.Location (Math|Transform|BreakTransform (Math|Transform|ComposeTransforms (Utilities|Array|Get(acopy) (Variables|Default|GetTransformList) _array_index) (Transformation|GetActorTransform)))))))

(fn GetManageCategory
  (return "NewEnumerator0"))