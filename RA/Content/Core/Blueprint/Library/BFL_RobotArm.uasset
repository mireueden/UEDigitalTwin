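; BFL_RobotArm is a Blueprint function library that gives global access to shared robot arm actors and managers.
; GetConveyorActor and GetRAManagerEx each cast the current game mode to BP_RAGameMode and return its ConveyorActor or RAManagreEx reference.
; If the cast fails, each function returns without setting a value.
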(fn GetConveyorActor
  (bind _asbp_ragame_mode (Utilities|Casting|CastToBP_RAGameMode (Game|GetGameMode))
    (:then
      (return (Variables|/Game/Core/Blueprint/GameMode/BP_RAGameMode.BP_RAGameMode_C|GetConveyorActor _asbp_ragame_mode)))
    (:CastFailed
      (return 0))))

(fn GetRAManagerEx
  (bind _asbp_ragame_mode (Utilities|Casting|CastToBP_RAGameMode (Game|GetGameMode))
    (:then
      (return (Variables|/Game/Core/Blueprint/GameMode/BP_RAGameMode.BP_RAGameMode_C|GetRAManagreEx _asbp_ragame_mode)))
    (:CastFailed
      (return 0))))