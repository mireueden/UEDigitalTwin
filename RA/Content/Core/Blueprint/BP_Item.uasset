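; BP_Item is an item actor that can be picked up, placed and assigned to a target spline.
; A guarded state setter fires OnItemStateChanged, and assigning or clearing the spline switches state unless one particular state is active.
; Pickup uses a mesh socket transform, while placement box-traces downward with the actor's bounds to find a resting location.
; The placement trace always draws debug shapes, and a separate helper visualizes and prints the result.
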(event EventBeginPlay)

(fn ConstructionScript)

(fn SetTargetSpline
  (params (TargetSpline :type Spline%20Component%20Object%20Reference))
  (if (Utilities|Enum|NotEqual(Enum) (Variables|Internal|GetItemState) "NewEnumerator1")
    (bind _output_get (Variables|Internal|SetTargetSpline TargetSpline))
    (CallFunction|SetItemState (select (Utilities|IsValid _output_get) "NewEnumerator2" "NewEnumerator0"))))

(fn GetTargetSpline
  (return (Variables|Internal|GetTargetSpline)))

(fn SetItemState
  (params (NewItemState :type E_ItemState%20Enum :default "NewEnumerator0"))
  (if (Utilities|Enum|NotEqual(Enum) NewItemState (Variables|Internal|GetItemState))
    (bind _output_get (LocalVariables|SetPrevState (Variables|Internal|GetItemState)))
    (bind _output_get_2 (Variables|Internal|SetItemState NewItemState))
    (Default|CallOnItemStateChanged _output_get _output_get_2)))

(fn GetItemState
  (return (Variables|Internal|GetItemState)))

(fn IsStateEquals
  (params (State :type E_ItemState%20Enum :default "NewEnumerator0"))
  (return (Utilities|Enum|Equal(Enum) State (Variables|Internal|GetItemState))))

(fn GetPickupTransform
  (params (TransformSpace :type ERelativeTransformSpace%20Enum :default "RTS_World"))
  (return (Transformation|GetSocketTransform (Variables|Default|GetMeshComponent) (Variables|Default|GetPickupSocketName) TransformSpace)))

(fn GetPlaceTransform
  (params (InTransform :type Transform))
  (bind _location (Math|Transform|BreakTransform InTransform))
  (bind (_location_2 _rotation _scale) (Math|Transform|BreakTransform InTransform))
  (bind (_outhit _returnvalue) (Class|KismetSystemLibrary|BoxTraceSinglebyProfile (+ _location "0.000000,0.000000,100.000000") _location (.BoxExtent (Collision|GetActorBounds false false)) "0, 0, 0" (Collision|GetCollisionProfileName (Variables|Default|GetMeshComponent)) false 0 "ForDuration" true))
  (if _returnvalue
    (return (Math|Transform|MakeTransform (.Location (Collision|BreakHitResult _outhit)) _rotation _scale))
    (else
      (return InTransform))))

(fn DebugPlaceTransform
  (bind _debugtransform (Variables|Debug|GetDebugTransform))
  (bind _outtransform (CallFunction|GetPlaceTransform _debugtransform))
  (bind (_location _rotation) (Math|Transform|BreakTransform _outtransform))
  (bind (_x _y _z) (Math|Vector|BreakVector _location))
  (Rendering|Debug|DrawDebugBox :Center _location :Extent (.BoxExtent (Collision|GetActorBounds false false)) :Rotation _rotation :Duration 5.0 :Thickness 2e+01)
  (Development|PrintText (Utilities|Text|FormatText "(X={X},Y={Y},Z={Z})" (Utilities|Text|ToText(Float) _x "HalfToEven" false false) (Utilities|Text|ToText(Float) _y "HalfToEven" false false) (Utilities|Text|ToText(Float) _z "HalfToEven" false false))))