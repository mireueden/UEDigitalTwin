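; BP_RAGameMode is the game mode for the RA mode, setting up references to its core level actors when play begins.
; It stores the first BP_ConveyorActor found in the level.
; It then synchronously loads the soft RAManagerExClass, spawns that manager at the world origin, and keeps a reference to it.
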(event Custom|InitReference
  (bind _ramanagerexclass (Variables|Default|GetRAManagerExClass))
  (Utilities|FlowControl|Sequence
    (:then_0
      (bind _outactors (Actor|GetAllActorsOfClass "/Game/Core/Blueprint/BP_ConveyorActor.BP_ConveyorActor_C"))
      (if (Utilities|Array|IsValidIndex _outactors)
        (Variables|Default|SetConveyorActor (Utilities|Array|Get(acopy) _outactors))))
    (:then_1
      (Utilities|LoadClassAssetBlocking _ramanagerexclass)
      (bind _returnvalue (Game|SpawnActorfromClass (Utilities|ResolveSoftReference _ramanagerexclass) (Math|Transform|MakeTransform "0, 0, 0") "Undefined" "MultiplyWithRoot" 0 0))
      (Variables|Default|SetRAManagreEx _returnvalue))))

(event EventBeginPlay
  (CallFunction|InitReference))

(fn ConstructionScript)