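; Manager actor that tracks manageable world actors and dispatches idle delivery bots to work.
; On BeginPlay it registers every BPI_Manage actor into a map of lists keyed by category.
; StartProcess pulls a bot from the first cargo BP_BotQueue, assigns the default work spec row, and re-arms itself on a random-interval timer until StopProcess clears it.
; It also provides lookups for category lists and non-full queues.
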(event Custom|StartProcess
  (bind _deliverybot (CallFunction|GetIdleDeliveryBotinCargo false))
  (Utilities|IsValid _deliverybot
    (:Is%20Valid
      (Utilities|FlowControl|Sequence
        (:then_0
          ;[0.15 0.15 0.15 0.5] 메뉴 UI 같은곳에서 스펙을 선택, 또는 외부에서 할당
          (bind _returnvalue (Utilities|GetDataTableRow "/Game/Core/Blueprint/Data/DT_WorkSpecTable.DT_WorkSpecTable" "Default")
            (:then
              (Default|AssignWork _deliverybot _returnvalue))))
        (:then_1
          (Utilities|Time|ClearandInvalidateTimerbyHandle (Variables|Default|GetProcessTimer) :!label _label)
          (bind _returnvalue_2 (Utilities|Time|SetTimerbyEvent (delegate Custom|StartProcess) (Math|Random|RandomFloatinRange 1.0 2.0) true))
          (Variables|Default|SetProcessTimer _returnvalue_2))))
    (:Is%20Not%20Valid
      (goto _label))))

(event Custom|StopProcess
  (Utilities|Time|ClearandInvalidateTimerbyHandle (Variables|Default|GetProcessTimer)))

(event EventBeginPlay
  (bind _outactors (Actor|GetAllActorswithInterface "/Game/Core/Blueprint/Interface/BPI_Manage.BPI_Manage_C"))
  (for _array_element _outactors
    (CallFunction|RegisterManageMap _array_element)))

(fn ConstructionScript)

(fn RegisterManageMap
  (params (ManageActor :type Actor%20Object%20Reference))
  (bind _managemap (Variables|Default|GetManageMap))
  (bind _category (Class|BPIManage|GetManageCategory(Message) ManageActor))
  (bind _output_get (LocalVariables|SetManageActorData (.Value (Utilities|Map|Find _managemap _category))))
  (Utilities|Array|Add (Utilities|Struct|BreakS_ManageActorsData _output_get) (.AsBPI%20Manage (Utilities|Casting|CastToBPI_Manage ManageActor)))
  (Utilities|Map|Add _managemap _category _output_get))

(fn GetManagerListbyType
  (params (Key :type E_RACategory%20Enum :default "NewEnumerator0"))
  (return (.Value (Utilities|Map|Find (Variables|Default|GetManageMap) Key))))

(fn GetIdleDeliveryBotinCargo
  (params (bCheckOnly :type Boolean))
  (bind _value (CallFunction|GetManagerListbyType "NewEnumerator4"))
  (bind _list (Utilities|Struct|BreakS_ManageActorsData _value))
  (if (Utilities|Array|IsValidIndex _list)
    (bind _asbp_bot_queue (Utilities|Casting|CastToBP_BotQueue (Utilities|ToObject(Interface) (Utilities|Array|Get(acopy) _list)))
      (:then
        (if bCheckOnly
          (bind _output (Default|Top _asbp_bot_queue))
          (return _output)
          (else
            (bind _output_get (Default|Dequeue _asbp_bot_queue))
            (return _output_get))))
      (:CastFailed
        (return 0)))))

(fn GetAvailabeQueuebyCategory
  (params (Category :type E_RACategory%20Enum :default "NewEnumerator0"))
  (Utilities|FlowControl|Sequence
    (:then_0
      (switch Utilities|FlowControl|Switch|SwitchonE_RACategory Category
        (:NewEnumerator1
          _)
        (:NewEnumerator3
          _)
        (:NewEnumerator4
          _))
      (bind _array_element (Utilities|Array|ForEachLoopwithBreak (Utilities|Struct|BreakS_ManageActorsData (CallFunction|GetManagerListbyType Category)) :!label _label)
        (:LoopBody
          (bind _asbp_bot_queue (Utilities|Casting|CastToBP_BotQueue _array_element))
          (bind _returnvalue (Default|IsQueueFull _asbp_bot_queue))
          (if (not _returnvalue)
            (LocalVariables|SetFondWork _asbp_bot_queue)
            (goto _label Break)))))
    (:then_1
      (return (LocalVariables|GetFondWork)))))