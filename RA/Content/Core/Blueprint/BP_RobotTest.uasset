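; BP_RobotTest is a test Blueprint that drives a robot skeletal mesh through a Control Rig, using a billboard as the target.
; On BeginPlay it maps the skeletal mesh to the rig as an output.
; Before each forward solve, it snaps the end control to the billboard's world transform.
; It also sets the A control's yaw from the mesh-to-billboard direction via MakeRotFromZ, keeping its roll and pitch.
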(event OnPreForwardsSolveDelegate(ControlRig)
  (params (Component :type Control%20Rig%20Component%20Object%20Reference))
  (bind _returnvalue (Class|ControlRigComponent|GetControlRotator Component "Robot1_A_ctrl" "WorldSpace"))
  (bind _billboard (Variables|Default|GetBillboard))
  (bind (_roll _pitch) (Math|Rotator|BreakRotator _returnvalue))
  (Utilities|FlowControl|Sequence
    (:then_0
      (Class|ControlRigComponent|SetControlTransform Component "Robot1_End_ctrl" (Transformation|GetWorldTransform _billboard) "WorldSpace"))
    (:then_1
      (Class|ControlRigComponent|SetControlRotator Component "Robot1_A_ctrl" (Math|Rotator|MakeRotator _roll _pitch (.Yaw (Math|Rotator|BreakRotator (Math|Rotator|MakeRotfromZ (- (Transformation|GetWorldLocation _billboard) (Transformation|GetWorldLocation (Variables|Default|GetSkeletalMesh))))))) "WorldSpace"))))

(event EventBeginPlay
  (Class|ControlRigComponent|AddMappedCompleteSkeletalMesh (Variables|Default|GetControlRig) (Variables|Default|GetSkeletalMesh) "Output"))

(fn ConstructionScript)