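; Spawner Blueprint for a UI example that creates the example HUD on BeginPlay and bulk-spawns items when Space Bar is pressed.
; Each press spawns 200 BP_Item actors at the player pawn's transform, each given a new BP_ItemData object with a sequential index and random color category.
; Spawned items accumulate in ItemList and are announced one by one through the OnItemSpawned dispatcher.
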(event EventBeginPlay
  (bind _returnvalue (UserInterface|CreateWidget "/Game/UIExample/Widget/WBP_UIExampleHUD.WBP_UIExampleHUD_C" (Game|GetPlayerController 0)))
  (UserInterface|Viewport|AddtoViewport _returnvalue 0))

(event Input|KeyboardEvents|SpaceBar
  (params (Key :type Key%20Structure :default "None"))
  (:Pressed
    (for _index (range 0 199)
      (bind _returnvalue (Game|ConstructObjectfromClass "/Game/UIExample/Blueprint/BP_ItemData.BP_ItemData_C" (+ (Utilities|Array|LastIndex (Variables|Default|GetItemList)) 1) (.OutItem (Utilities|Array|Random (Utilities|Array|MakeArray "Red" "Green" "Blue" "Yellow")))))
      (bind _returnvalue_2 (Game|SpawnActorfromClass "/Game/UIExample/Blueprint/BP_Item.BP_Item_C" (Transformation|GetActorTransform (Game|Player|GetPlayerPawn 0)) "Undefined" "MultiplyWithRoot" 0 _returnvalue 0))
      (Utilities|Array|Add (Variables|Default|GetItemList) _returnvalue_2)
      (Default|CallOnItemSpawned _returnvalue_2))))

(fn ConstructionScript)