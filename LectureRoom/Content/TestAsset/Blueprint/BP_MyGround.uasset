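; Test ground actor that spawns a handful of balls at random points inside its box and periodically scatters them.
; BeginPlay calls SpawnBall in a loop, then starts a looping timer that fires ShuffleBall every few seconds.
; ShuffleBall moves each entry in BallList through SetBallLocation.
; Both spawn and shuffle take positions from GetRandomLocationInBound, which samples the Box component's scaled world-space extent.
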(event Custom|ShuffleBall
  (for _array_element (Variables|Default|GetBallList)
    (Class|MyBall|SetBallLocation _array_element (CallFunction|GetRandomLocationinBound))))

(event EventBeginPlay
  (for _index (range 0 4)
    (Class|MyGround|SpawnBall (Math|Transform|MakeTransform (CallFunction|GetRandomLocationinBound))))
  (Utilities|Time|SetTimerbyEvent (delegate Custom|ShuffleBall) 3.0 true))

(fn ConstructionScript)

(fn GetRandomLocationinBound
  (bind _box (Variables|Default|GetBox))
  (return (Math|Random|RandomPointinBoundingBox (Transformation|GetWorldLocation _box) (Components|Box|GetScaledBoxExtent _box))))