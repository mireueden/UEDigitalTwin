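; BP_Apple is an apple actor that takes its mesh from AppleData and stops simulating physics shortly after its first hit.
; On BeginPlay it applies the mesh and fits the Sphere collision radius to the mesh bounds, or prints a missing-mesh message.
; The first Sphere hit, gated by DoOnce, starts a short timer that turns off physics simulation on the Sphere.
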(event OnComponentHit(Sphere)
  (params (HitComponent :type Primitive%20Component%20Object%20Reference) (OtherActor :type Actor%20Object%20Reference) (OtherComp :type Primitive%20Component%20Object%20Reference) (NormalImpulse :type Vector :default "0, 0, 0") (Hit :type Hit%20Result%20Structure%20%28by%20ref%29))
  (Utilities|FlowControl|DoOnce false
    (:Completed
      (Utilities|Time|SetTimerbyEvent (delegate Custom|DisablePhysics) 2.0))))

(event Custom|DisablePhysics
  (Physics|SetSimulatePhysics (Variables|Default|GetSphere) false))

(event EventBeginPlay
  (bind _staticmesh (Variables|Default|GetStaticMesh))
  (bind _appledata (Variables|Default|GetAppleData))
  (Utilities|IsValid (.mesh _appledata)
    (:Is%20Valid
      (Components|StaticMesh|SetStaticMesh _staticmesh (.mesh _appledata))
      (Components|Sphere|SetSphereRadius (Variables|Default|GetSphere) (.SphereRadius (Collision|GetComponentBounds _staticmesh)) true))
    (:Is%20Not%20Valid
      (Development|PrintString "사과 메시가 없습니다." true true "(R=1.000000,G=0.000000,B=0.000000,A=1.000000)"))))

(fn ConstructionScript)