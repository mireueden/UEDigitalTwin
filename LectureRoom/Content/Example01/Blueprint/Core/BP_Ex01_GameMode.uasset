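; Game mode that spawns and registers a configurable list of manager actors, starting on each PostLogin.
; It walks the soft class list recursively, async-loading, spawning and attaching each manager in turn while skipping invalid references.
; Spawned managers are mapped by class for GetManagerByClass lookup.
; InitializedManagers is set after a one-second delay; the Finish notification fires at the start and Start at the end.
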(event Custom|SpawnManagerClassAtIndex
  (params (Index :type Integer))
  (bind _managerclasslist (Variables|Default|GetManagerClassList))
  (bind _output (Utilities|Array|Get(acopy) _managerclasslist Index))
  (bind _output_2 (Utilities|ResolveSoftReference _output))
  (if (Utilities|Array|IsValidIndex _managerclasslist Index)
    (if (Utilities|IsValidSoftClassReference _output)
      (Utilities|AsyncLoadClassAsset _output
        (:Completed
          (bind _returnvalue (Game|SpawnActorfromClass _output_2 (Math|Transform|MakeTransform "0, 0, 0") "AlwaysSpawn" "MultiplyWithRoot" 0 0))
          (Utilities|FlowControl|Sequence
            (:then_0
              (Utilities|Map|Add (Variables|Default|GetManagerTypeRefereceMap) (Utilities|ResolveSoftReference _output_2) _returnvalue))
            (:then_1
              (Transformation|AttachActorToActor _returnvalue self "None" "KeepRelative" "KeepRelative" "KeepRelative" true))
            (:then_2
              (CallFunction|TrySpawnManageratIndex)))))
      (else
        (CallFunction|TrySpawnManageratIndex)))
    (else
      (CallFunction|FinishSpawnManagers))))

(event Custom|TrySpawnManagerAtIndex
  (CallFunction|SpawnManagerClassatIndex (+ (stale Custom|SpawnManagerClassAtIndex Index) 1)))

(event Custom|SpawnManagers
  (Variables|Default|SetbInitializedManagers false)
  (Default|CallOnFinishSpawnManagers)
  (CallFunction|SpawnManagerClassatIndex))

(event Custom|FinishSpawnManagers
  (Utilities|FlowControl|Delay 1.0)
  (Variables|Default|SetbInitializedManagers true)
  (Default|CallOnStartSpawnManagers))

(event EventPostLogin
  (params (NewPlayer :type Player%20Controller%20Object%20Reference))
  (CallFunction|SpawnManagers))

(fn ConstructionScript)

(fn GetManagerbyClass
  (params (Key :type BP%20Ex%2001%20Manager%20Base%20Soft%20Class%20Reference%20%28by%20ref%29))
  (return (.Value (Utilities|Map|Find (Variables|Default|GetManagerTypeRefereceMap) Key))))