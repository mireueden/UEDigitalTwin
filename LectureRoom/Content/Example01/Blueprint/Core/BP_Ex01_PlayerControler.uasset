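; Player controller for Example01 that holds the screen black at startup and manages the HUD widget.
; BeginPlay blacks out camera and audio, then re-arms a short timer until BP_Ex01_GameMode reports its managers initialized, and only then clears the fade and shows the HUD.
; ShowHUD lazily creates WBP_Ex01_HUD on first use, and HideHUD hides the existing widget.
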(event Custom|HideHUD
  (bind _hudwidget (Variables|Default|GetHUDWidget)
    (:then
      (Default|HideHUD _hudwidget))
    (:else)))

(event Custom|ShowHUD
  (Variables|Default|GetHUDWidget
    (:then
      _)
    (:else
      (bind _returnvalue (UserInterface|CreateWidget "/Game/Example01/Widget/WBP_Ex01_HUD.WBP_Ex01_HUD_C" self))
      (bind _output_get (Variables|Default|SetHUDWidget _returnvalue))
      (UserInterface|Viewport|AddtoViewport _output_get 0)))
  (Default|ShowHUD (Variables|Default|GetHUDWidget)))

(event Custom|WaitInitializeManager
  (if (Variables|/Game/Example01/Blueprint/Core/BP_Ex01_GameMode.BP_Ex01_GameMode_C|GetbInitializedManagers (stale EventBeginPlay _asbp_ex_01_game_mode))
    (Class|PlayerCameraManager|SetManualCameraFade :self (Variables|Default|GetPlayerCameraManager))
    (CallFunction|ShowHUD)
    (else
      (Utilities|Time|SetTimerbyEvent (delegate Custom|WaitInitializeManager) 0.1))))

(event EventBeginPlay
  (Utilities|FlowControl|Sequence
    (:then_0
      (Class|PlayerCameraManager|SetManualCameraFade :self (Variables|Default|GetPlayerCameraManager) :InFadeAmount 1.0 :bInFadeAudio true))
    (:then_1
      (bind _asbp_ex_01_game_mode (Utilities|Casting|CastToBP_Ex01_GameMode (Game|GetGameMode)))
      (if (Variables|/Game/Example01/Blueprint/Core/BP_Ex01_GameMode.BP_Ex01_GameMode_C|GetbInitializedManagers _asbp_ex_01_game_mode)
        (Class|PlayerCameraManager|SetManualCameraFade :self (Variables|Default|GetPlayerCameraManager))
        (CallFunction|ShowHUD)
        (else
          (Utilities|Time|SetTimerbyEvent (delegate Custom|WaitInitializeManager) 0.1))))))

(fn ConstructionScript)