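; BP_Ex01_CameraActor is an interaction target that offers a list of switchable camera viewpoints with captured images.
; CollectCameraActors fills that list from directly attached CameraActors.
; After BeginPlay waits for game mode managers, one shared SceneCapture2D snapshots each camera into its own render target, then the actor registers with the interaction manager until EndPlay.
; SetViewPointbyIndex blends the player's view to a chosen camera, while getters expose viewpoint count and textures.
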(event Custom|WaitInitializeManagers
  (if (Variables|/Game/Example01/Blueprint/Core/BP_Ex01_GameMode.BP_Ex01_GameMode_C|GetbInitializedManagers (stale EventBeginPlay _asbp_ex_01_game_mode))
    (CallFunction|InitRenderTarget)
    (bind _manager (CallFunction|GetEx01ManagerInteraction))
    (Default|AddInteractionTarget _manager self)
    (else
      (Utilities|Time|SetTimerbyEvent (delegate Custom|WaitInitializeManagers) 0.1))))

(event EventBeginPlay
  (bind _asbp_ex_01_game_mode (Utilities|Casting|CastToBP_Ex01_GameMode (Game|GetGameMode)))
  (if (Variables|/Game/Example01/Blueprint/Core/BP_Ex01_GameMode.BP_Ex01_GameMode_C|GetbInitializedManagers _asbp_ex_01_game_mode)
    (CallFunction|InitRenderTarget)
    (bind _manager (CallFunction|GetEx01ManagerInteraction))
    (Default|AddInteractionTarget _manager self)
    (else
      (Utilities|Time|SetTimerbyEvent (delegate Custom|WaitInitializeManagers) 0.1))))

(event EventSetViewPointbyIndex
  (params (ViewIndex :type Integer))
  (bind _cameralist (Variables|Default|GetCameraList))
  (if (Utilities|Array|IsValidIndex _cameralist ViewIndex)
    (Game|Player|SetViewTargetwithBlend (Game|GetPlayerController 0) (Utilities|Array|Get(acopy) _cameralist ViewIndex) 0.2 "VTBlend_Linear" 0.0 false)))

(event EventEndPlay
  (params (EndPlayReason :type EEndPlayReason%20Enum :default "Destroyed"))
  (bind _manager (CallFunction|GetEx01ManagerInteraction))
  (Utilities|IsValid _manager
    (:Is%20Valid
      (Default|RemoveInteractionTarget _manager self))))

(fn ConstructionScript)

(fn CollectCameraActors
  (bind _cameralist (Variables|Default|GetCameraList))
  (Utilities|FlowControl|Sequence
    (:then_0
      (Utilities|Array|Clear _cameralist))
    (:then_1
      (for _array_element (Actor|GetAttachedActors true false)
        (bind _ascamera_actor (Utilities|Casting|CastToCameraActor _array_element))
        (Utilities|Array|Add _cameralist _ascamera_actor)))))

(fn InitRenderTarget
  (for (_ _array_index) (Variables|Default|GetCameraList)
    (Utilities|FlowControl|Sequence
      (:then_0
        (bind _returnvalue (Rendering|CreateRenderTarget2D 256 256 "RTF_RGBA16f"))
        (Utilities|Array|Add (Variables|Default|GetTextureRenderTargetList) _returnvalue)
        (Variables|/Script/Engine.SceneCaptureComponent2D|SetTextureTarget (Variables|Default|GetSceneCaptureComponent2D) _returnvalue))
      (:then_1
        (CallFunction|CaptureRenderTargetforCamera _array_index)))))

(fn CaptureRenderTargetforCamera
  (params (CameraIndex :type Integer))
  (bind _scenecapturecomponent2d (Variables|Default|GetSceneCaptureComponent2D))
  (bind _cameralist (Variables|Default|GetCameraList))
  (if (Utilities|Array|IsValidIndex _cameralist CameraIndex)
    (bind _output_get (Variables|/Script/Engine.SceneCaptureComponent2D|SetTextureTarget _scenecapturecomponent2d (CallFunction|GetTextureRenderTarget CameraIndex)))
    (Utilities|IsValid _output_get
      (:Is%20Valid
        (CallFunction|CopySceneCaptureSettingsfromCamera _scenecapturecomponent2d (Variables|/Script/Engine.CameraActor|GetCameraComponent (Utilities|Array|Get(acopy) _cameralist CameraIndex)))
        (Rendering|SceneCapture|CaptureScene _scenecapturecomponent2d :!class /Script/Engine.SceneCaptureComponent2D)))))

(fn GetTextureRenderTarget
  (params (Index :type Integer))
  (bind _texturerendertargetlist (Variables|Default|GetTextureRenderTargetList))
  (if (Utilities|Array|IsValidIndex _texturerendertargetlist Index)
    (return (Utilities|Array|Get(acopy) _texturerendertargetlist Index))
    (else
      (return 0))))

(fn CanCameraInteraction
  (return (Utilities|Array|IsNotEmpty (Variables|Default|GetCameraList))))

(fn GetViewPointCount
  (return (Utilities|Array|Length (Variables|Default|GetCameraList))))

(fn GetViewpointTexturebyIndex
  (params (Index :type Integer))
  (return (CallFunction|GetTextureRenderTarget Index)))