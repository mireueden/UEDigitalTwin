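; Interaction manager for Example01 that tracks a list of interactable targets and the currently selected one.
; Adding, removing and changing targets fire notification calls, while next and previous selection wrap around the list by index.
; View point switching, view point count and camera-interaction checks are forwarded to the current target through an interface.
; View out clears the selection index and blends the player's view target; the viewpoint texture getter is an empty stub.
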(event EventSetViewPointbyIndex
  (params (ViewIndex :type Integer))
  (bind _target (Variables|Default|GetTarget))
  (if (Utilities|IsValidInterface _target)
    (Default|SetViewPointbyIndex _target ViewIndex)))

(fn ConstructionScript
  (|CallParentFunction))

(fn SetInteractionTarget
  (params (NewTarget :type BPI%20Ex%2001%20Interactable%20Interface))
  (if (!= (Utilities|ToObject(Interface) (Variables|Default|GetTarget)) (Utilities|ToObject(Interface) NewTarget))
    (LocalVariables|SetPrevTarget (Variables|Default|GetTarget))
    (bind _output_get (Variables|Default|SetTarget NewTarget))
    (Default|CallOnTargetChanged (LocalVariables|GetPrevTarget) (Variables|Default|GetTarget))))

(fn GetCurrentTarget
  (return (Variables|Default|GetTarget)))

(fn AddInteractionTarget
  (params (NewItem :type BPI%20Ex%2001%20Interactable%20Interface%20%28by%20ref%29))
  (if (Utilities|IsValidInterface NewItem)
    (Utilities|Array|Add (Variables|Default|GetInteractionList) NewItem)
    (Default|CallOnTargetAdded NewItem)))

(fn RemoveInteractionTarget
  (params (Item :type BPI%20Ex%2001%20Interactable%20Interface%20%28by%20ref%29))
  (Utilities|Array|RemoveItem (Variables|Default|GetInteractionList) Item)
  (Default|CallOnTargetRemoved Item))

(fn NextInteractionTarget
  (bind _interactionlist (Variables|Default|GetInteractionList))
  (if (> (Utilities|Array|Length _interactionlist) 1)
    (bind _output_get (LocalVariables|SetNextIndex (+ (Variables|Default|GetSelectIndex) 1)))
    (CallFunction|TrySetSelect (Math|Integer|SelectInt _output_get 0 (Utilities|Array|IsValidIndex _interactionlist _output_get)))))

(fn PrevinteractionTarget
  (bind _interactionlist (Variables|Default|GetInteractionList))
  (if (> (Utilities|Array|Length _interactionlist) 1)
    (bind _output_get (LocalVariables|SetPrevIndex (+ (Variables|Default|GetSelectIndex) -1)))
    (bind _returnvalue (CallFunction|TrySetSelect (Math|Integer|SelectInt _output_get (Utilities|Array|LastIndex _interactionlist) (Utilities|Array|IsValidIndex _interactionlist _output_get))))
    (if _returnvalue
      (CallFunction|SetInteractionTarget (Utilities|Array|Get(acopy) _interactionlist (Math|Integer|SelectInt _output_get (Utilities|Array|LastIndex _interactionlist) (Utilities|Array|IsValidIndex _interactionlist _output_get)))))))

(fn TrySetSelect
  (params (SelectIndex :type Integer))
  (if (!= SelectIndex (Variables|Default|GetSelectIndex))
    (CallFunction|SetSelect SelectIndex)
    (return true)
    (else
      (return false))))

(fn SetSelect
  (params (SelectIndex :type Integer))
  (bind _interactionlist (Variables|Default|GetInteractionList))
  (bind _output_get (Variables|Default|SetSelectIndex (select (Utilities|Array|IsValidIndex _interactionlist SelectIndex) SelectIndex -1)))
  (CallFunction|SetInteractionTarget (Utilities|Array|Get(acopy) _interactionlist _output_get)))

(fn SetViewin
  (params (bNewTarget :type Boolean))
  (if (Utilities|IsValidInterface (Variables|Default|GetTarget))
    (CallFunction|SetInteractionTarget (Variables|Default|GetTarget))
    (elif bNewTarget
      (CallFunction|TrySetSelect))))

(fn SetViewOut
  (CallFunction|SetSelect -1)
  (Game|Player|SetViewTargetwithBlend (Game|GetPlayerController 0) 0 0.2 "VTBlend_Linear" 0.0 false))

(fn CanCameraInteraction
  (bind _target (Variables|Default|GetTarget))
  (if (Utilities|IsValidInterface _target)
    (bind _benable (Default|CanCameraInteraction _target))
    (return _benable)
    (else
      (return false))))

(fn GetViewPointCount
  (bind _target (Variables|Default|GetTarget))
  (if (Utilities|IsValidInterface _target)
    (bind _count (Default|GetViewPointCount _target))
    (return _count)
    (else
      (return 0))))

(fn GetViewpointTexturebyIndex
  (params (Index :type Integer))
  (return 0))