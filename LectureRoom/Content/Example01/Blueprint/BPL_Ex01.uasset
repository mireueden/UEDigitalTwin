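; Blueprint function library of shared helpers for Example01.
; GetEx01ManagerInteraction looks up the interaction manager through BP_Ex01_GameMode's GetManagerByClass and returns it cast to BP_Ex01Manager_Interaction, or empty if the game mode cast fails.
; CopySceneCaptureSettingsFromCamera matches a scene capture to a camera by teleporting it to the camera's world transform and copying its field of view, after checking both components are valid.
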(fn GetEx01ManagerInteraction
  (bind _asbp_ex_01_game_mode (Utilities|Casting|CastToBP_Ex01_GameMode (Game|GetGameMode))
    (:then
      (bind _value (Default|GetManagerbyClass _asbp_ex_01_game_mode (LocalVariables|GetManagerClass)))
      (return (.AsBP%20Ex%2001Manager%20Interaction (Utilities|Casting|CastToBP_Ex01Manager_Interaction _value))))
    (:CastFailed
      (return 0))))

(fn CopySceneCaptureSettingsfromCamera
  (params (SceneCapture2DComp :type Scene%20Capture%20Component%202D%20Object%20Reference) (CameraComp :type Camera%20Component%20Object%20Reference))
  (Utilities|IsValid CameraComp
    (:Is%20Valid
      (Utilities|IsValid SceneCapture2DComp
        (:Is%20Valid
          (Transformation|SetWorldTransform SceneCapture2DComp (Transformation|GetWorldTransform CameraComp) false true)
          (Variables|/Script/Engine.SceneCaptureComponent2D|SetFOVAngle SceneCapture2DComp (Variables|/Script/Engine.CameraComponent|GetFieldOfView CameraComp)))))))