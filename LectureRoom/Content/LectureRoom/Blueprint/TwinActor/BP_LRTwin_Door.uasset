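; BP_LRTwin_Door is a lecture room door that swings open when a controlled pawn enters its trigger volume and closes when one leaves.
; The construction script offsets the mesh and collision to hinge at the actor origin and takes the attach-parent TriggerVolume as trigger.
; Overlap events bound at BeginPlay play or reverse a yaw-lerping timeline.
; A right-vector dot product on the pawn's side of the trigger picks swing direction.
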(event Custom|Bind
  (bind _trigger (Variables|Default|GetTrigger)
    (:then
      (Collision|BindEventtoOnActorBeginOverlap _trigger (delegate Custom|OnBeginOverlapTrigger))
      (Collision|BindEventtoOnActorEndOverlap _trigger (delegate Custom|OnEndOverlapTrigger)))
    (:else)))

(event Custom|OnBeginOverlapTrigger
  (params (OverlappedActor :type Actor%20Object%20Reference) (OtherActor :type Actor%20Object%20Reference))
  (bind _aspawn (Utilities|Casting|CastToPawn OtherActor))
  (if (Class|Pawn|IsControlled _aspawn)
    (bind _bright (CallFunction|GetEnterDirection OverlappedActor OtherActor))
    (bind _rate (Timeline|Timeline Play)
      (:Update
        (Transformation|SetActorRotation (Math|Rotator|MakeRotator 0.0 0.0 (Math|Float|Lerp (Variables|Default|GetBaseYaw) (* (Variables|Default|GetDeltaYaw) (Math|Float|SelectFloat -1.0 1.0 _bright)) _rate)) true)))))

(event Custom|OnEndOverlapTrigger
  (params (OverlappedActor :type Actor%20Object%20Reference) (OtherActor :type Actor%20Object%20Reference))
  (bind _aspawn (Utilities|Casting|CastToPawn OtherActor))
  (if (Class|Pawn|IsControlled _aspawn)
    (bind _rate (Timeline|Timeline Reverse)
      (:Update
        (Transformation|SetActorRotation (Math|Rotator|MakeRotator 0.0 0.0 (Math|Float|Lerp (Variables|Default|GetBaseYaw) (* (Variables|Default|GetDeltaYaw) (Math|Float|SelectFloat -1.0 1.0 (stale Custom|OnBeginOverlapTrigger _bright))) _rate)) true)))))

(event Custom|Unbind
  (bind _trigger (Variables|Default|GetTrigger)
    (:then
      (Collision|UnbindEventfromOnActorBeginOverlap _trigger (EventDispatchers|CreateEvent :!event Custom|OnBeginOverlapTrigger))
      (EventDispatchers|UnbindEventfromOnActorEndOverlap _trigger (EventDispatchers|CreateEvent :!event Custom|OnEndOverlapTrigger)))
    (:else)))

(event EventBeginPlay
  (|CallParentFunction)
  (CallFunction|Bind))

(event EventEndPlay
  (params (EndPlayReason :type EEndPlayReason%20Enum :default "Destroyed"))
  (CallFunction|Unbind))

(fn ConstructionScript
  (bind _door (Variables|Default|GetDoor))
  (|CallParentFunction)
  (Utilities|FlowControl|Sequence
    (:then_0
      (Transformation|SetRelativeLocation (Variables|Default|GetCollisionComp) (Math|Vector|MakeVectorNetQuantize (.X (Math|Vector|BreakVector (.BoxExtent (Collision|GetComponentBounds _door)))) 0.0 0.0) false true)
      (Transformation|SetRelativeScale3D (Variables|Default|GetCollisionComp) (/ (Variables|/Script/Engine.SceneComponent|GetRelativeScale3D _door) 2)))
    (:then_1
      (bind _astrigger_volume (Utilities|Casting|CastToTriggerVolume (Actor|GetAttachParentActor)))
      (Variables|Default|SetTrigger _astrigger_volume))))

(fn GetEnterDirection
  (params (EnteringActor :type Actor%20Object%20Reference) (TriggerActor :type Actor%20Object%20Reference))
  (return (> (Math|Vector|DotProduct (Transformation|GetActorRightVector) (- (Transformation|GetActorLocation TriggerActor) (Transformation|GetActorLocation EnteringActor))) 0.0)))