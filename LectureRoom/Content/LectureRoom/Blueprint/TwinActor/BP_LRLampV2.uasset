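; BP_LRLampV2 is a lecture room lamp twin actor that can be switched on and off.
; Construction creates a dynamic material instance on the CylinderLamp mesh's first material slot.
; Turnon and TurnOff call the parent events, then set the light intensity to full or zero.
; UpdateLampLight pushes intensity and color into the material's parameters, so the visible change is driven through the material.
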(event EventTurnOff
  (|CallParentFunction)
  (Variables|Default|SetLightIntensity 0.0)
  (CallFunction|UpdateLampLight))

(event EventTurnon
  (|CallParentFunction)
  (Variables|Default|SetLightIntensity 1.0)
  (CallFunction|UpdateLampLight))

(fn ConstructionScript
  (bind _cylinder_lamp (Variables|Default|GetCylinder_Lamp))
  (|CallParentFunction)
  (bind _returnvalue (Rendering|Material|CreateDynamicMaterialInstance _cylinder_lamp 0 (Rendering|Material|GetMaterial _cylinder_lamp 0) "None" :!class /Script/Engine.PrimitiveComponent))
  (Variables|Default|SetLampMID _returnvalue)
  (CallFunction|UpdateLampLight))

(fn UpdateLampLight
  (bind _lampmid (Variables|Default|GetLampMID)
    (:then
      (Rendering|Material|SetScalarParameterValue _lampmid "Intensity" (Variables|Default|GetLightIntensity) :!class /Script/Engine.MaterialInstanceDynamic)
      (Rendering|Material|SetVectorParameterValue _lampmid "Color" (Variables|Default|GetLightColor) :!class /Script/Engine.MaterialInstanceDynamic))
    (:else)))