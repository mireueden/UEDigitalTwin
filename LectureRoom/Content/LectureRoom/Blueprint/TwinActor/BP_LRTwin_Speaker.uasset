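; BP_LRTwin_Speaker is a speaker twin actor for the lecture room that can be switched on and off.
; It extends the parent's Turnon and TurnOff events, calling the parent first, then activating (with reset) or deactivating its Niagara effect and MediaSound components together.
; BeginPlay is a disabled stub and the construction script only calls the parent, so it adds no other logic.
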(event EventBeginPlay
  (|CallParentFunction) ; This node is disabled and will not be called.\nDrag off pins to build functionality.
)

(event EventTurnon
  (|CallParentFunction)
  (Components|Activation|Activate (Variables|Default|GetNiagara) true))

(event EventTurnOff
  (|CallParentFunction)
  (Components|Activation|Deactivate (Variables|Default|GetNiagara)))

(fn ConstructionScript
  (|CallParentFunction))