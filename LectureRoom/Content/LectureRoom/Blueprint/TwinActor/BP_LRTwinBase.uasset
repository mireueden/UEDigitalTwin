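; Base actor for interactable "Twin" objects in the lecture room, with an on/off state and focus feedback.
; On BeginPlay it initializes its LR interact component and syncs the on/off state from whether that component is working.
; Turning on or off swaps the image on its WBP_Interact widget.
; Focus toggles the widget's visibility, its focus animation and a custom depth stencil outline on all mesh components.
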(event Custom|SetOutlineMesh
  (params (bEnable :type Boolean))
  (bind _returnvalue (CallFunction|GetMeshComponents))
  (if (Utilities|Array|IsNotEmpty _returnvalue)
    (Rendering|SetRenderCustomDepth _returnvalue bEnable)
    (Rendering|SetCustomDepthStencilValue _returnvalue (Math|Integer|SelectInt 255 0 bEnable))))

(event EventBeginPlay
  (Utilities|FlowControl|Sequence
    (:then_0
      (bind _asbp_lrinteract_component (Utilities|Casting|CastToBP_LRInteractComponent (Variables|Default|GetLRComponent)))
      (Default|InitInstance _asbp_lrinteract_component))
    (:then_1
      (if (Class|LRInteractComponentBase|IsWorking (Variables|Default|GetLRComponent))
        (Class|LRActorInterface|Turnon)
        (else
          (Class|LRActorInterface|TurnOff))))))

(event EventTurnon
  (bind _interactwidget (Utilities|GetInteractWidget)
    (:then
      (Default|SetImageon _interactwidget))))

(event EventTurnOff
  (bind _interactwidget (Utilities|GetInteractWidget)
    (:then
      (Default|SetImageOff _interactwidget))))

(event EventBeginFocus
  (Rendering|SetVisibility (Variables|Default|GetWidget) true false)
  (CallFunction|SetOutlineMesh true)
  (bind _interactwidget (Utilities|GetInteractWidget)
    (:then
      (Default|PlayFocusAnimation _interactwidget))))

(event EventEndFocus
  (Rendering|SetVisibility (Variables|Default|GetWidget) false false)
  (CallFunction|SetOutlineMesh false)
  (bind _interactwidget (Utilities|GetInteractWidget)
    (:then
      (Default|StopFocusAnimation _interactwidget))))

(fn ConstructionScript)

(fn GetMeshComponents
  (return (Actor|GetComponentsByClass self "/Script/Engine.MeshComponent")))