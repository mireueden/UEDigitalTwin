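; BP_LRScreen is a lecture room screen twin actor that plays video when turned on and pauses it when turned off.
; It opens the media source at BeginPlay, tracks readiness through the player's opened and closed events, and unbinds them at EndPlay.
; Turning on before the media is ready starts a short timer that retries until playback can start.
; A dynamic material created in the construction script toggles its IsMedia parameter with playback.
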(event Custom|WaitMediaReady
  (if (Variables|Default|GetbReadyMedia)
    (Media|MediaPlayer|Play (Variables|Default|GetMediaPlayer) :!class /Script/MediaAssets.MediaPlayer)
    (Rendering|Material|SetScalarParameterValue (Variables|Default|GetVideoMID) "IsMedia" 1.0 :!class /Script/Engine.MaterialInstanceDynamic)
    (elif (not (Utilities|Time|IsTimerActivebyHandle (Variables|Default|GetWaitMediaReadyTimer)))
      (bind _returnvalue (Utilities|Time|SetTimerbyEvent (delegate Custom|WaitMediaReady) 0.1))
      (Variables|Default|SetWaitMediaReadyTimer _returnvalue))))

(event EventBeginPlay
  (|CallParentFunction)
  (CallFunction|Bind))

(event EventEndPlay
  (params (EndPlayReason :type EEndPlayReason%20Enum :default "Destroyed"))
  (Utilities|FlowControl|Sequence
    (:then_0
      (CallFunction|Unbind))
    (:then_1
      (|CallParentFunction EndPlayReason))))

(event EventTurnon
  (|CallParentFunction)
  (if (Variables|Default|GetbReadyMedia)
    (Media|MediaPlayer|Play (Variables|Default|GetMediaPlayer) :!class /Script/MediaAssets.MediaPlayer)
    (Rendering|Material|SetScalarParameterValue (Variables|Default|GetVideoMID) "IsMedia" 1.0 :!class /Script/Engine.MaterialInstanceDynamic)
    (elif (not (Utilities|Time|IsTimerActivebyHandle (Variables|Default|GetWaitMediaReadyTimer)))
      (bind _returnvalue (Utilities|Time|SetTimerbyEvent (delegate Custom|WaitMediaReady) 0.1))
      (Variables|Default|SetWaitMediaReadyTimer _returnvalue))))

(event EventTurnOff
  (|CallParentFunction)
  (if (Variables|Default|GetbReadyMedia)
    (Sequencer|Player|Pause (Variables|Default|GetMediaPlayer))
    (Rendering|Material|SetScalarParameterValue (Variables|Default|GetVideoMID) "IsMedia" 0.0 :!class /Script/Engine.MaterialInstanceDynamic)))

(fn ConstructionScript
  (bind _staticmeshcomponent0 (Variables|Default|GetStaticMeshComponent0))
  (if (== (Variables|Default|GetVideoMID) 0)
    (bind _returnvalue (Rendering|Material|CreateDynamicMaterialInstance _staticmeshcomponent0 0 (Rendering|Material|GetMaterial _staticmeshcomponent0 0) "None" :!class /Script/Engine.PrimitiveComponent))
    (bind _output_get (Variables|Default|SetVideoMID _returnvalue))
    (Rendering|Material|SetMaterial (Variables|Default|GetStaticMeshComponent0) 0 _output_get)))

(fn Unbind
  (bind _mediaplayer (Variables|Default|GetMediaPlayer))
  (Media|MediaPlayer|UnbindEventfromOnMediaOpened _mediaplayer (EventDispatchers|CreateEvent :!event OnMediaOpened))
  (Media|MediaPlayer|UnbindEventfromOnMediaClosed _mediaplayer (EventDispatchers|CreateEvent :!event OnMediaClosed)))

(fn Bind
  (bind _mediaplayer (Variables|Default|GetMediaPlayer))
  (Media|MediaPlayer|BindEventtoOnMediaOpened _mediaplayer (EventDispatchers|CreateEvent :!event OnMediaOpened))
  (Media|MediaPlayer|BindEventtoOnMediaClosed _mediaplayer (EventDispatchers|CreateEvent :!event OnMediaClosed))
  (Media|MediaPlayer|OpenSourcewithOptions (Variables|Default|GetMediaPlayer) (Variables|Default|GetMediaSource) (Utilities|Struct|MakeMediaPlayerOptions "(Audio=0,Caption=-1,Metadata=-1,Script=-1,Subtitle=-1,Text=-1,Video=0)" "(Video=\"\",Audio=\"\",Subtitle=\"\",Caption=\"\")" "UseTrackOptionIndices" "+00000000.00:00:00.000000000" "RelativeToStartTime" "Disabled" "Enabled") :!class /Script/MediaAssets.MediaPlayer))

(fn OnMediaOpened
  (params (OpenedUrl :type String))
  (Variables|Default|SetbReadyMedia true))

(fn OnMediaClosed
  (Variables|Default|SetbReadyMedia false))