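; BP_LRTwin_BeamProjector is a lecture room twin actor for a beam projector that switches its linked screen along with itself.
; TurnOn and TurnOff run the parent behavior, then forward the same call to the LRComponent of ScreenActor when that reference is valid.
; The construction script only calls the parent's, leaving disconnected nodes that would fit CollisionComp to the skeletal mesh bounds.
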(event EventTurnon
  (|CallParentFunction)
  (bind _screenactor (Variables|Default|GetScreenActor)
    (:then
      (Class|LRInteractComponentBase|Turnon (Variables|/Script/DT.LRInteractiveActor|GetLRComponent _screenactor)))
    (:else)))

(event EventTurnOff
  (|CallParentFunction)
  (bind _screenactor (Variables|Default|GetScreenActor)
    (:then
      (Class|LRInteractComponentBase|TurnOff (Variables|/Script/DT.LRInteractiveActor|GetLRComponent _screenactor)))
    (:else)))

(fn ConstructionScript
  (|CallParentFunction))