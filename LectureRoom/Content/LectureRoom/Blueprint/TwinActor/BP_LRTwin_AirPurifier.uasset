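; BP_LRTwin_AirPurifier is a lecture-room twin actor for an air purifier that shows an intake effect while switched on.
; It extends its parent's turn-on and turn-off events.
; Turning on spawns the NS_AirIntake Niagara system, unattached, at the mesh's air_intake socket location and stores the component.
; Turning off deactivates that component if valid, prints a validity check and clears the reference.
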(event EventBeginPlay
  (|CallParentFunction) ; This node is disabled and will not be called.\nDrag off pins to build functionality.
)

(event EventTurnon
  (|CallParentFunction)
  (bind _returnvalue (Niagara|SpawnSystematLocation "/Game/LectureRoom/VFX/NS_AirIntake.NS_AirIntake" (Transformation|GetSocketLocation (Variables|Default|GetStaticMesh) "air_intake")))
  (Variables|Default|SetIntakeEffectComp _returnvalue))

(event EventTurnOff
  (|CallParentFunction)
  (bind _intakeeffectcomp (Variables|Default|GetIntakeEffectComp)
    (:then
      (Components|Activation|Deactivate _intakeeffectcomp)
      (Development|PrintString (Utilities|String|ToString(Boolean) (Utilities|IsValid (Variables|Default|GetIntakeEffectComp))))
      (Variables|Default|SetIntakeEffectComp 0))
    (:else)))

(fn ConstructionScript
  (|CallParentFunction))