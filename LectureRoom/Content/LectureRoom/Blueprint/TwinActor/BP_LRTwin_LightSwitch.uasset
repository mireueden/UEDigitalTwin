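; Light switch twin actor for the lecture room that turns a set of linked interactive actors on and off.
; On BeginPlay it syncs to its LRComponent working state.
; TurnOn and TurnOff tilt the switch mesh in opposite yaw directions and forward the call to each LRComponent in InteractionList.
; RefreshInteractionList rebuilds that list from LRInteractiveActor instances carrying FindInteractionTag.
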(event EventBeginPlay
  (|CallParentFunction)
  (if (Class|LRInteractComponentBase|IsWorking (Variables|Default|GetLRComponent))
    (Class|LRActorInterface|Turnon)
    (else
      (Class|LRActorInterface|TurnOff))))

(event EventTurnOff
  (|CallParentFunction)
  (Transformation|SetRelativeRotation (Variables|Default|GetCube_Switch) (Math|Rotator|MakeRotator 0.0 0.0 1e+01) false false)
  (for _array_element (Variables|Default|GetInteractionList)
    (Class|LRInteractComponentBase|TurnOff (Variables|/Script/NSDT.LRInteractiveActor|GetLRComponent _array_element))))

(event EventTurnon
  (|CallParentFunction)
  (Transformation|SetRelativeRotation (Variables|Default|GetCube_Switch) (Math|Rotator|MakeRotator 0.0 0.0 -1e+01) false false)
  (for _array_element (Variables|Default|GetInteractionList)
    (Class|LRInteractComponentBase|Turnon (Variables|/Script/NSDT.LRInteractiveActor|GetLRComponent _array_element))))

(fn ConstructionScript
  (|CallParentFunction))

(fn RefreshInteractionList
  (bind _interactionlist (Variables|Default|GetInteractionList))
  (bind _outactors (Actor|GetAllActorsOfClasswithTag "/Script/NSDT.LRInteractiveActor" (Variables|Default|GetFindInteractionTag)))
  (Utilities|FlowControl|Sequence
    (:then_0
      (Utilities|Array|Clear _interactionlist))
    (:then_1
      (Utilities|Array|AppendArray _interactionlist _outactors))))