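; Lecture room interaction component that gives an object a twin-data instance and an ID.
; InitInstance, when TwinDataAsset is valid, constructs an LRTwinData object, sets its ID from TwinObjectId, then initializes it from the asset.
; GetID exposes TwinObjectId, and an author note flags that ID validity is not yet guaranteed during initialization.
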(event EventBeginPlay)

(event EventTick
  (params (DeltaSeconds :type Float%20%28single-precision%29)))

(fn InitInstance
  (bind _twindataasset (Variables|Default|GetTwinDataAsset))
  (Utilities|IsValid _twindataasset
    (:Is%20Valid
      (bind _returnvalue (Game|ConstructObjectfromClass "/Script/DT.LRTwinData"))
      (bind _output_get (Variables|Default|SetTwinData _returnvalue))
      ;[0.15 0.15 0.15 0.5] Id 유효한 상태가 보장할 수 있도록 로직 개선 필요
      (Utilities|FlowControl|Sequence
        (:then_0
          (Class|LRTwinData|SetId _output_get (Variables|Default|GetTwinObjectId)))
        (:then_1
          (Class|LRTwinData|InitTwinData _output_get _twindataasset))))))

(fn GetID
  (return (Variables|Default|GetTwinObjectId)))