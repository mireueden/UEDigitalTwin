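; Spline-based conveyor that carries BP_Apple actors along its path.
; The construction script tiles visual and lowered collision instanced meshes along the spline, spaced by the mesh's X bounds.
; Collision overlaps add apples to a list, which Tick moves by MoveSpeed along the nearest spline direction, taken in local space.
; On end overlap, apples leave the list and get a near-zero lifespan, destroying them.
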(event OnComponentBeginOverlap(InstancedStaticMesh_Collision)
  (params (OverlappedComponent :type Primitive%20Component%20Object%20Reference) (OtherActor :type Actor%20Object%20Reference) (OtherComp :type Primitive%20Component%20Object%20Reference) (OtherBodyIndex :type Integer) (bFromSweep :type Boolean) (SweepResult :type Hit%20Result%20Structure%20%28by%20ref%29))
  (Utilities|IsValid OtherActor
    (:Is%20Valid
      (if (Utilities|ClassIsChildOf (Utilities|GetClass OtherActor) "/Game/AppleTwin/Blueprint/BP_Apple.BP_Apple_C")
        (bind _asbp_apple (Utilities|Casting|CastToBP_Apple OtherActor))
        (Utilities|Array|Add (Variables|Default|GetAppleList) _asbp_apple)))))

(event OnComponentEndOverlap(InstancedStaticMesh_Collision)
  (params (OverlappedComponent :type Primitive%20Component%20Object%20Reference) (OtherActor :type Actor%20Object%20Reference) (OtherComp :type Primitive%20Component%20Object%20Reference) (OtherBodyIndex :type Integer))
  (bind _applelist (Variables|Default|GetAppleList))
  (bind _asbp_apple (Utilities|Casting|CastToBP_Apple OtherActor))
  (if (Utilities|Array|ContainsItem _applelist _asbp_apple)
    (Utilities|Array|RemoveItem _applelist _asbp_apple)
    (Actor|SetLifeSpan _asbp_apple 0.01)))

(event EventBeginPlay)

(event Collision|EventActorBeginOverlap
  (params (OtherActor :type Actor%20Object%20Reference)))

(event EventTick
  (params (DeltaSeconds :type Float%20%28single-precision%29))
  (for _array_element (Variables|Default|GetAppleList)
    (Transformation|AddActorWorldOffset _array_element (* (Spline|FindDirectionClosesttoWorldLocation (Variables|Default|GetSpline) (Transformation|GetActorLocation _array_element) "Local") (* (Variables|Default|GetMoveSpeed) DeltaSeconds)))))

(fn ConstructionScript
  (bind _new_mesh (Variables|Default|GetNew%20Mesh))
  (bind _spline (Variables|Default|GetSpline))
  (bind _returnvalue (StaticMesh|GetBoundingBox _new_mesh))
  (bind _returnvalue_2 (Spline|GetSplineLength _spline))
  (bind (_min _max) (Utilities|Struct|BreakBox _returnvalue))
  (bind _returnvalue_3 (- _max _min))
  (bind _x (Math|Vector|BreakVector _returnvalue_3))
  (bind _returnvalue_4 (/ _returnvalue_2 _x))
  (bind _returnvalue_5 (Math|Float|Floor _returnvalue_4))
  (Components|StaticMesh|SetStaticMesh (Variables|Default|GetInstancedStaticMesh) _new_mesh)
  (Variables|Default|SetSpacing _x)
  (LocalVariables|SetNumInstances _returnvalue_5)
  (for _index (range 0 _returnvalue_5)
    (Components|InstancedStaticMesh|AddInstance (Variables|Default|GetInstancedStaticMesh) (CallFunction|GetLocationbySplineDistance _index "0, 0, 0") false)
    (Components|InstancedStaticMesh|AddInstance (Variables|Default|GetInstancedStaticMesh_Collision) (CallFunction|GetLocationbySplineDistance _index "0.000000,0.000000,-60.000000") false)))

(fn GetLocationbySplineDistance
  (params (Index :type Integer) (Offset :type Vector))
  (bind _spline (Variables|Default|GetSpline))
  (bind _spacing (Variables|Default|GetSpacing))
  (bind _returnvalue (* Index _spacing))
  (bind _returnvalue_2 (Spline|GetLocationatDistanceAlongSpline _spline _returnvalue "Local"))
  (return (Math|Transform|MakeTransform (+ Offset _returnvalue_2) (Math|Rotator|MakeRotfromX (- (Spline|GetLocationatDistanceAlongSpline _spline (* (+ Index 1) _spacing) "Local") _returnvalue_2)))))