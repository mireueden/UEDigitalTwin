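; BP_AppleSpawner spawns an apple with random data, position and rotation each time Space is pressed.
; The key event picks a random row name from AppleDataTable and a random point within the SpawnVolume actor's bounds.
; SpawnApple looks up that row and spawns BP_Apple with it as AppleData.
; An older StaticMeshActor spawning path remains, deprecated and disconnected.
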(event EventBeginPlay)

(event Input|KeyboardEvents|SpaceBar
  (params (Key :type Key%20Structure :default "None"))
  (bind _spawnvolume (Variables|Default|GetSpawnVolume))
  (bind _appledatatable (Variables|Default|GetAppleDataTable))
  (bind (_origin _boxextent) (Collision|GetActorBounds _spawnvolume false false))
  (:Pressed
    (Utilities|IsValid _appledatatable
      (:Is%20Valid
        (bind _outrownames (DataTable|GetDataTableRowNames _appledatatable))
        (Apple|SpawnApple (Math|Transform|MakeTransform (Math|Random|RandomPointinBoundingBox _origin _boxextent) (Math|Random|RandomRotator true)) (.OutItem (Utilities|Array|Random _outrownames)))))))

(fn ConstructionScript)

(fn SpawnApple
  (params (SpawnTransform :type Transform) (RowName :type Name))
  (bind _returnvalue (Utilities|GetDataTableRow (Variables|Default|GetAppleDataTable) RowName)
    (:then
      (Game|SpawnActorfromClass "/Game/AppleTwin/Blueprint/BP_Apple.BP_Apple_C" SpawnTransform "Undefined" "MultiplyWithRoot" 0 _returnvalue 0))))