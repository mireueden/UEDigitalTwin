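; Player pawn for the lecture room, moved by Enhanced Input, with mouse X turning it and mouse Y zooming a spring arm whose pitch follows its length.
; Holding IA_Function adds a UI mapping context.
; Overlaps retarget among LRInteractiveActors, and a timeline magnets the pawn onto the target's XY bounds center.
; The nearest-target search compares the pawn's location with itself, so the first overlapping actor always wins.
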(event OnComponentBeginOverlap(CollisionComp)
  (params (OverlappedComponent :type Primitive%20Component%20Object%20Reference) (OtherActor :type Actor%20Object%20Reference) (OtherComp :type Primitive%20Component%20Object%20Reference) (OtherBodyIndex :type Integer) (bFromSweep :type Boolean) (SweepResult :type Hit%20Result%20Structure%20%28by%20ref%29))
  (Development|PrintString (Utilities|String|Append "LRPawn BeginOverlap : " (Utilities|GetDisplayName OtherActor) " / " (Utilities|GetDisplayName OtherComp))))

(event Custom|ChangeTargetArmLength
  (params (Target%20Arm%20Length :type Float%20%28single-precision%29))
  (bind _springarmcomp (Variables|Default|GetSpringArmComp))
  (Utilities|FlowControl|Sequence
    (:then_0
      (Components|Timeline|SetPlayRate (Variables|Default|GetZooming) (/ 1.0 (Variables|Default|GetZoomingTime))))
    (:then_1
      (bind _rate (Timeline|Zooming PlayFromStart)
        (:Update
          (bind _output_get (Variables|/Script/Engine.SpringArmComponent|SetTargetArmLength _springarmcomp (Math|Float|Lerp (Variables|/Script/Engine.SpringArmComponent|GetTargetArmLength _springarmcomp) Target%20Arm%20Length _rate)))
          (Transformation|SetRelativeRotation _springarmcomp (Math|Rotator|MakeRotator 0.0 (Math|Float|MapRangeClamped _output_get 7e+02 2e+03 -9e+01 -75.0) 0.0) false false))))))

(event Custom|MagnetToTarget
  (bind _returnvalue (Transformation|GetActorLocation))
  (bind _targetingactor (Variables|Default|GetTargetingActor))
  (bind _origin (Collision|GetActorBounds _targetingactor true false))
  (bind (_x _y) (Math|Vector|BreakVector _origin))
  (Utilities|IsValid _targetingactor
    (:Is%20Valid
      (bind _rate (Timeline|Timeline PlayFromStart)
        (:Update
          (Transformation|SetActorLocation (Math|Vector|Lerp(Vector) _returnvalue (Math|Vector|MakeVector _x _y (.Z (Math|Vector|BreakVector _returnvalue))) _rate) false true))))))

(event EventPossessed
  (params (NewController :type Controller%20Object%20Reference))
  (bind _asplayer_controller (Utilities|Casting|CastToPlayerController NewController))
  (Input|AddMappingContext (PlayerController|LocalPlayerSubsystems|GetEnhancedInputLocalPlayerSubsystem _asplayer_controller) "/Game/LectureRoom/Input/IMC_Default.IMC_Default" 0 (Utilities|Struct|MakeModifyContextOptions true false false)))

(event Collision|EventActorBeginOverlap
  (params (OtherActor :type Actor%20Object%20Reference))
  (CallFunction|UpdateTargetingActor OtherActor))

(event Collision|EventActorEndOverlap
  (params (OtherActor :type Actor%20Object%20Reference))
  (CallFunction|UpdateTargetingActor OtherActor))

(event EventTick
  (params (DeltaSeconds :type Float%20%28single-precision%29)))

(event EventUnpossessed
  (params (OldController :type Controller%20Object%20Reference))
  (bind _asplayer_controller (Utilities|Casting|CastToPlayerController OldController))
  (Input|RemoveMappingContext (PlayerController|LocalPlayerSubsystems|GetEnhancedInputLocalPlayerSubsystem _asplayer_controller) "/Game/LectureRoom/Input/IMC_Default.IMC_Default" "(bIgnoreAllPressedKeysUntilRelease=True,bForceImmediately=False,bNotifyUserSettings=False)"))

(event Input|EnhancedActionEvents|EnhancedInputActionIA_Move
  (params (ActionValue :type Vector%202D%20Structure) (ElapsedSeconds :type Float%20%28double-precision%29) (TriggeredSeconds :type Float%20%28double-precision%29) (InputAction :type Input%20Action%20Object%20Reference :default "/Game/LectureRoom/Input/IA_Move.IA_Move"))
  (bind (_x _y) (Math|Vector2D|BreakVector2D ActionValue))
  (:Triggered
    (Utilities|FlowControl|Sequence
      (:then_0
        (Class|PawnMovementComponent|AddInputVector (Variables|Default|GetMovementComp) (* (Math|Vector|RotateVector (Math|Conversions|ToVector(Vector2D) (Math|Vector2D|MakeVector2D _y _x)) (Pawn|GetControlRotation :!class /Script/Engine.Pawn)) (Variables|Default|GetMoveSpped)) false))
      (:then_1
        (|DebugMessage ActionValue :!label _label))))
  (:Started
    (goto _label execute5))
  (:Ongoing
    (goto _label execute4))
  (:Canceled
    (goto _label execute3))
  (:Completed
    (goto _label execute2)))

(event Input|EnhancedActionEvents|EnhancedInputActionIA_Function
  (params (ActionValue :type Boolean) (ElapsedSeconds :type Float%20%28double-precision%29) (TriggeredSeconds :type Float%20%28double-precision%29) (InputAction :type Input%20Action%20Object%20Reference :default "/Game/LectureRoom/Input/IA_Function.IA_Function"))
  (bind _returnvalue (Pawn|GetController))
  (:Triggered
    ;[0.15 0.15 0.15 0.5] Pressed /Release
    (if ActionValue
      (bind _asplayer_controller (Utilities|Casting|CastToPlayerController _returnvalue))
      (Input|AddMappingContext (PlayerController|LocalPlayerSubsystems|GetEnhancedInputLocalPlayerSubsystem _asplayer_controller) "/Game/LectureRoom/Input/IMC_UI_Default.IMC_UI_Default" 0 "(bIgnoreAllPressedKeysUntilRelease=True,bForceImmediately=False,bNotifyUserSettings=False)")
      (else
        (bind _asplayer_controller_2 (Utilities|Casting|CastToPlayerController _returnvalue))
        (Input|RemoveMappingContext (PlayerController|LocalPlayerSubsystems|GetEnhancedInputLocalPlayerSubsystem _asplayer_controller_2) "/Game/LectureRoom/Input/IMC_UI_Default.IMC_UI_Default" "(bIgnoreAllPressedKeysUntilRelease=True,bForceImmediately=False,bNotifyUserSettings=False)")))))

(event Input|EnhancedActionEvents|EnhancedInputActionIA_MouseMove
  (params (ActionValue :type Vector%202D%20Structure) (ElapsedSeconds :type Float%20%28double-precision%29) (TriggeredSeconds :type Float%20%28double-precision%29) (InputAction :type Input%20Action%20Object%20Reference :default "/Game/LectureRoom/Input/IA_MouseMove.IA_MouseMove"))
  (bind (_x _y) (Math|Vector2D|BreakVector2D ActionValue))
  (:Triggered
    (Utilities|FlowControl|Sequence
      (:then_0
        (Pawn|Input|AddControllerYawInput _x)
        (Transformation|SetActorRotation (Pawn|GetControlRotation :!class /Script/Engine.Pawn) true))
      (:then_1
        (if (> (Math|Float|Absolute(Float) _y) 0.0)
          (CallFunction|ChangeTargetArmLength (Math|Float|Clamp(Float) (+ (* _y (Variables|Default|GetZoomSpeed)) (Variables|/Script/Engine.SpringArmComponent|GetTargetArmLength (Variables|Default|GetSpringArmComp))) 7e+02 2e+03)))))))

(fn ConstructionScript)

(fn UpdateTargetingActor
  (params (NewTarget :type Actor%20Object%20Reference))
  (bind _returnvalue (Transformation|GetActorLocation))
  (bind _returnvalue_2 (Transformation|GetActorLocation))
  (bind _returnvalue_3 (Class|KismetMathLibrary|VectorDistanceSquared _returnvalue_2 _returnvalue))
  (bind _output_get (LocalVariables|SetNewLocalVar (Collision|GetOverlappingActors "/Script/DT.LRInteractiveActor" :!class /Script/Engine.Actor)))
  (if (> (Utilities|Array|Length _output_get) 0)
    (for (_array_element _array_index) _output_get
      (if (== _array_index 0)
        (LocalVariables|SetMinDistanceTarget _array_element)
        (LocalVariables|SetMinDistanceSquared _returnvalue_3)
        (elif (> (LocalVariables|GetMinDistanceSquared) _returnvalue_3)
          (LocalVariables|SetMinDistanceTarget _array_element)
          (LocalVariables|SetMinDistanceSquared _returnvalue_3))))
    (CallFunction|SetTargetingActor (LocalVariables|GetMinDistanceTarget))
    (else
      (CallFunction|SetTargetingActor))))

(fn SetTargetingActor
  (params (NewTarget :type Actor%20Object%20Reference))
  (if (!= NewTarget (Variables|Default|GetTargetingActor))
    (bind _output_get (Variables|Default|SetTargetingActor NewTarget))
    (Utilities|FlowControl|Sequence
      (:then_0
        (Utilities|IsValid _output_get
          (:Is%20Valid
            (CallFunction|MagnettoTarget))
          (:Is%20Not%20Valid
            (Audio|Components|Audio|Stop (Variables|Default|GetTimeline)))))
      (:then_1
        (Default|CallOnTargetingChanged _output_get)))))