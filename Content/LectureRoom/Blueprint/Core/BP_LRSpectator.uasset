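; BP_LRSpectator is the player's spectator pawn in the lecture room, with Enhanced Input look and movement and cursor-based targeting of interactive actors.
; Each tick it traces objects under the cursor, updates the target, reports changes to the World Twin Manager, and prints the target's name.
; Left click toggles the target's LRComponent on or off when its interaction type is GameOnly or GameAndUI.
; Possession and unpossession add and remove the input mapping context.
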(event Input|EnhancedActionEvents|EnhancedInputActionIA_MouseLB
  (params (ActionValue :type Boolean) (ElapsedSeconds :type Float%20%28double-precision%29) (TriggeredSeconds :type Float%20%28double-precision%29) (InputAction :type Input%20Action%20Object%20Reference :default "/Game/LectureRoom/Input/IA_MouseLB.IA_MouseLB"))
  (bind _target_actor (Variables|Default|GetTarget%20Actor)
    (:then
      (if (Utilities|Set|Contains (Utilities|Set|MakeSet "GameOnly" "GameAndUI") (Class|LRLibrary|GetInteractionType (Variables|/Script/DT.LRInteractiveActor|GetLRComponent _target_actor)))
        (if (Class|LRInteractComponentBase|IsWorking (Variables|/Script/DT.LRInteractiveActor|GetLRComponent _target_actor))
          (Class|LRInteractComponentBase|TurnOff (Variables|/Script/DT.LRInteractiveActor|GetLRComponent _target_actor))
          (else
            (Class|LRInteractComponentBase|Turnon (Variables|/Script/DT.LRInteractiveActor|GetLRComponent _target_actor))))))
    (:else)))

(event Input|EnhancedActionEvents|EnhancedInputActionIA_MouseMove
  (params (ActionValue :type Vector%202D%20Structure) (ElapsedSeconds :type Float%20%28double-precision%29) (TriggeredSeconds :type Float%20%28double-precision%29) (InputAction :type Input%20Action%20Object%20Reference :default "/Game/LectureRoom/Input/IA_MouseMove.IA_MouseMove"))
  (bind (_x _y) (Math|Vector2D|BreakVector2D ActionValue))
  (Pawn|Input|AddControllerPitchInput _y)
  (Pawn|Input|AddControllerYawInput _x))

(event Input|EnhancedActionEvents|EnhancedInputActionIA_Move
  (params (ActionValue :type Vector%202D%20Structure) (ElapsedSeconds :type Float%20%28double-precision%29) (TriggeredSeconds :type Float%20%28double-precision%29) (InputAction :type Input%20Action%20Object%20Reference :default "/Game/LectureRoom/Input/IA_Move.IA_Move"))
  (bind (_x _y) (Math|Vector2D|BreakVector2D ActionValue))
  (Class|PawnMovementComponent|AddInputVector (Variables|Default|GetMovement) (Math|Vector|RotateVector (Math|Conversions|ToVector(Vector2D) (Math|Vector2D|MakeVector2D _y _x)) (Pawn|GetControlRotation :!class /Script/Engine.Pawn)) false))

(event EventTick
  (params (DeltaSeconds :type Float%20%28single-precision%29))
  (bind _cachedlrplayercontroller (Variables|Default|GetCachedLRPlayerController)
    (:then
      (if (.ReturnValue (Class|PlayerController|GetHitResultUnderCursorforObjects _cachedlrplayercontroller (Utilities|Array|MakeArray "ObjectTypeQuery7") false))
        (bind _aslrinteractive_actor (Utilities|Casting|CastToLRInteractiveActor (.HitActor (Collision|BreakHitResult (.HitResult (Class|PlayerController|GetHitResultUnderCursorforObjects _cachedlrplayercontroller (Utilities|Array|MakeArray "ObjectTypeQuery7") false))))))
        (CallFunction|TryChangeTargetActor _aslrinteractive_actor)
        (Development|PrintString (Utilities|GetDisplayName _aslrinteractive_actor) true false "(R=0.144796,G=0.000000,B=1.000000,A=1.000000)" 0.0)
        (else
          (CallFunction|TryChangeTargetActor))))
    (:else)))

(event EventPossessed
  (params (NewController :type Controller%20Object%20Reference))
  (bind _asbp_lrplayer_controller (Utilities|Casting|CastToBP_LRPlayerController NewController))
  (bind _output_get (Variables|Default|SetCachedLRPlayerController _asbp_lrplayer_controller))
  (Input|AddMappingContext (PlayerController|LocalPlayerSubsystems|GetEnhancedInputLocalPlayerSubsystem _output_get) "/Game/LectureRoom/Input/IMC_Default.IMC_Default" 0 "(bIgnoreAllPressedKeysUntilRelease=True,bForceImmediately=False,bNotifyUserSettings=False)"))

(event EventUnpossessed
  (params (OldController :type Controller%20Object%20Reference))
  (bind _asbp_lrplayer_controller (Utilities|Casting|CastToBP_LRPlayerController OldController))
  (bind _output_get (Variables|Default|SetCachedLRPlayerController _asbp_lrplayer_controller))
  (Input|RemoveMappingContext (PlayerController|LocalPlayerSubsystems|GetEnhancedInputLocalPlayerSubsystem _output_get) "/Game/LectureRoom/Input/IMC_Default.IMC_Default" "(bIgnoreAllPressedKeysUntilRelease=True,bForceImmediately=False,bNotifyUserSettings=False)"))

(fn ConstructionScript)

(fn TryChangeTargetActor
  (params (NewTargetActor :type LR%20Interactive%20Actor%20Object%20Reference))
  (if (!= NewTargetActor (Variables|Default|GetTarget%20Actor))
    (LocalVariables|SetPrevLocalVar (Variables|Default|GetTarget%20Actor))
    (Variables|Default|SetTarget%20Actor NewTargetActor)
    (bind _returnvalue (Class|LRTwinManager|GetWorldTwinManager false))
    (Class|LRTwinManager|NotifyChangeTargetActor _returnvalue (LocalVariables|GetPrevLocalVar) (Variables|Default|GetTarget%20Actor))))