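; BP_LRLamp is a lecture room lamp actor that toggles a spotlight and mirrors its state on an icon widget.
; On BeginPlay it turns on or off according to its BPLRInteractComponent's working state.
; TurnOn and TurnOff set the spotlight visibility and the icon image, while BeginFocus and EndFocus play and stop the icon's focus animation.
; GetLampWidget casts the widget component's content to WBP_LampIcon for these calls.
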(event EventBeginPlay
  (if (Class|LRInteractComponentBase|IsWorking (Variables|Default|GetBP_LRInteractComponent))
    (Class|LRActorInterface|Turnon)
    (else
      (Class|LRActorInterface|TurnOff))))

(event Collision|EventActorBeginOverlap
  (params (OtherActor :type Actor%20Object%20Reference)))

(event EventTick
  (params (DeltaSeconds :type Float%20%28single-precision%29)))

(event EventTurnOff
  (Rendering|SetVisibility (Variables|Default|GetSpotLight) false false)
  (bind _aswbp_lamp_icon (Utilities|GetLampWidget)
    (:then
      (Default|SetImageOff _aswbp_lamp_icon))))

(event EventTurnon
  (Rendering|SetVisibility (Variables|Default|GetSpotLight) true false)
  (bind _aswbp_lamp_icon (Utilities|GetLampWidget)
    (:then
      (Default|SetImageon _aswbp_lamp_icon))))

(event EventEndFocus
  (bind _aswbp_lamp_icon (Utilities|GetLampWidget)
    (:then
      (Default|StopFocusAnimation _aswbp_lamp_icon))))

(event EventBeginFocus
  (bind _aswbp_lamp_icon (Utilities|GetLampWidget)
    (:then
      (Default|PlayFocusAnimation _aswbp_lamp_icon))))

(fn ConstructionScript)