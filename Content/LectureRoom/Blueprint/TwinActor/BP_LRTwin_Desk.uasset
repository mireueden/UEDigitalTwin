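; Lecture room twin-actor desk that slides its hanging monitor along local Z when turned on or off.
; Turn-on and turn-off call the parent logic, then MoveMonitor drives a timeline that interpolates the monitor across MonitorMoveAmount.
; The timeline play rate is scaled so the move takes MonitorMoveTime, falling back to normal speed for non-positive values.
; An Initialized flag makes state changes during parent BeginPlay snap instantly instead of animating.
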(event Custom|UpdateMonitorMoveTimelineRate
  (bind _monitormovetime (Variables|Default|GetMonitorMoveTime))
  (bind _monitormovetimeline (Variables|Default|GetMonitorMoveTimeline))
  (if (> _monitormovetime 0.0)
    (Components|Timeline|SetPlayRate _monitormovetimeline (/ (Components|Timeline|GetTimelineLength _monitormovetimeline) _monitormovetime))
    (else
      ;[0.15 0.15 0.15 0.5] 0보다 작은값이 들어오면
      ; 1배속 재생하도록 설정
      (Components|Timeline|SetPlayRate _monitormovetimeline 1.0))))

(event Custom|MoveMonitor
  (params (bEnabled :type Boolean) (bImmediately :type Boolean))
  (if bImmediately
    (CallFunction|SetMonitorLocation (Math|Conversions|ToFloat(Boolean) bEnabled))
    (else
      (CallFunction|UpdateMonitorMoveTimelineRate)
      (if bEnabled
        (bind (_direction _rate) (Timeline|MonitorMoveTimeline Play)
          (:Update
            (CallFunction|SetMonitorLocation _rate))
          (:Finished
            (CallFunction|SetMonitorLocation (Utilities|Select :Index _direction :Forward 1.0 :Backward 0.0))))
        (else
          (Timeline|MonitorMoveTimeline Reverse))))))

(event EventBeginPlay
  (Utilities|FlowControl|Sequence
    (:then_0
      (Variables|Default|SetbInitialized false))
    (:then_1
      (|CallParentFunction)
      (Variables|Default|SetbInitialized true))))

(event EventTurnon
  (|CallParentFunction)
  (CallFunction|MoveMonitor true (not (Variables|Default|GetbInitialized))))

(event EventTurnOff
  (|CallParentFunction)
  (CallFunction|MoveMonitor false (not (Variables|Default|GetbInitialized))))

(fn ConstructionScript
  (|CallParentFunction))

(fn SetMonitorLocation
  (params (Alpha :type Float%20%28double-precision%29))
  (bind _returnvalue (Math|Float|MakeLiteralFloat 5.0))
  (bind _sm_hangingmonitor_r (Variables|Default|GetSM_HangingMonitor_R))
  (bind _relativelocation (Variables|/Script/Engine.SceneComponent|GetRelativeLocation _sm_hangingmonitor_r))
  (bind (_x _y) (Math|Vector|BreakVector _relativelocation))
  (Transformation|SetRelativeLocation _sm_hangingmonitor_r (Math|Vector|MakeVector _x _y (Math|Float|Lerp _returnvalue (+ _returnvalue (Variables|Default|GetMonitorMoveAmount)) (Math|Float|Clamp(Float) Alpha))) false true))