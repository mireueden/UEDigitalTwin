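; BP_LRComputerComponent is a component for computers in the lecture room that enlarges its owning actor while that actor has focus.
; BeginPlay caches the owner's original scale.
; BeginFocus scales the owner up by half again, and EndFocus restores the cached scale.
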(event EventBeginPlay
  (Variables|Default|SetOwnerActorScale (Transformation|GetActorScale3D (Components|GetOwner))))

(event EventTick
  (params (DeltaSeconds :type Float%20%28single-precision%29)))

(event EventBeginFocus
  (Transformation|SetActorScale3D (Components|GetOwner) (* (Variables|Default|GetOwnerActorScale) 1.5)))

(event EventEndFocus
  (Transformation|SetActorScale3D (Components|GetOwner) (Variables|Default|GetOwnerActorScale)))