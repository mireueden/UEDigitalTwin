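; Test actor for visualizing collision trace results in the LectureRoom project.
; Every Tick it runs a single capsule trace by object type between points from MakeTraceParam, drawn for one frame.
; On a hit, DrawDebugTraceCapsule draws capsules at both Location and ImpactPoint in different colors, showing how they differ.
; Channel-based capsule, line and multi-line trace variants remain in the graph but are disconnected and never run.
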(event EventBeginPlay)

(event Collision|EventActorBeginOverlap
  (params (OtherActor :type Actor%20Object%20Reference)))

(event EventTick
  (params (DeltaSeconds :type Float%20%28single-precision%29))
  (bind (_startlocation _endlocation) (Utilities|MakeTraceParam))
  (bind (_outhit _returnvalue) (Class|KismetSystemLibrary|CapsuleTraceSingleforObjects _startlocation _endlocation (Variables|Default|GetRadius) (Variables|Default|GetHalf%20Height) (Utilities|Array|MakeArray (Variables|Default|GetObjectChannel)) false 0 "ForOneFrame" true))
  (Utilities|DrawDebugTraceCapsule _outhit _returnvalue))

(fn ConstructionScript)