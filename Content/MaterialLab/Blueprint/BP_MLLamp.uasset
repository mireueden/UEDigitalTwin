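; BP_MLLamp is a Material Lab lamp actor whose light material is configured in the Construction Script.
; With UseMPC on, it assigns the MI_LampLight_MPC material instance to LampLight, presumably for shared parameter-collection control.
; Otherwise it creates a dynamic material instance and writes the Color and Emissive variables to its LightColor and LightEmissive parameters.
; The event graph holds no active logic.
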(event EventBeginPlay)

(event Collision|EventActorBeginOverlap
  (params (OtherActor :type Actor%20Object%20Reference)))

(event EventTick
  (params (DeltaSeconds :type Float%20%28single-precision%29)))

(fn ConstructionScript
  (bind _lamplight (Variables|Default|GetLampLight))
  (if (Variables|Default|GetbUseMPC)
    (Rendering|Material|SetMaterial (Variables|Default|GetLampLight) 0 "/Game/MaterialLab/Material/MI_LampLight_MPC.MI_LampLight_MPC")
    (else
      (bind _returnvalue (Rendering|Material|CreateDynamicMaterialInstance _lamplight 0 0 "None" :!class /Script/Engine.PrimitiveComponent))
      (bind _output_get (Variables|Default|SetLampMID _returnvalue))
      (Rendering|Material|SetMaterial _lamplight 0 _output_get)
      (Rendering|Material|SetVectorParameterValue (Variables|Default|GetLampMID) "LightColor" (Variables|Default|GetColor) :!class /Script/Engine.MaterialInstanceDynamic)
      (Rendering|Material|SetScalarParameterValue (Variables|Default|GetLampMID) "LightEmissive" (Variables|Default|GetEmissive) :!class /Script/Engine.MaterialInstanceDynamic))))