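; Digital-twin keyboard key actor that animates its press and release when the incoming key matches its KeyInfo.
; PressKey plays and ReleaseKey reverses a Timeline that offsets the actor from its start location along its up vector.
; Timeline event tracks call the OnPressedVK and OnReleasedVK dispatchers with location and key, using two cross-resetting DoOnce gates so each fires once per transition.
; Disconnected Delay, timer and construction experiments remain unused.
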(event Custom|CustomEvent
  ;[0.15 0.15 0.15 0.5] Delay보다 제어가 가능한 Timer 사용을 권장합니다
)

(event Custom|ReleaseKey
  (params (Key :type Key%20Structure :default "None"))
  (bind _returnvalue (Transformation|GetActorLocation))
  (bind _keyinfo (Variables|Default|GetKeyInfo))
  (if (== Key (Variables|Default|GetKeyInfo))
    (bind _rate (Timeline|Timeline Reverse)
      (:Update
        (Transformation|SetActorLocation (+ (Variables|Default|GetBaseLocation) (* _rate (Variables|Default|GetOffset) (Transformation|GetActorUpVector))) false true))
      (:Pressed
        (Utilities|FlowControl|Sequence
          (:then_0
            (Utilities|FlowControl|DoOnce false :!label _label
              (:Completed
                (Default|CallOnPressedVK _returnvalue _keyinfo))))
          (:then_1
            (goto _label_2 Reset))))
      (:Released
        (Utilities|FlowControl|Sequence
          (:then_0
            (Utilities|FlowControl|DoOnce false :!label _label_2
              (:Completed
                (Default|CallOnReleasedVK _returnvalue _keyinfo))))
          (:then_1
            (goto _label Reset)))))))

(event Custom|PressKey
  (params (Key :type Key%20Structure :default "None"))
  (bind _returnvalue (Transformation|GetActorLocation))
  (bind _keyinfo (Variables|Default|GetKeyInfo))
  (if (== Key (Variables|Default|GetKeyInfo))
    (bind _rate (Timeline|Timeline Play)
      (:Update
        (Transformation|SetActorLocation (+ (Variables|Default|GetBaseLocation) (* _rate (Variables|Default|GetOffset) (Transformation|GetActorUpVector))) false true))
      (:Pressed
        (Utilities|FlowControl|Sequence
          (:then_0
            (Utilities|FlowControl|DoOnce false :!label _label
              (:Completed
                (Default|CallOnPressedVK _returnvalue _keyinfo))))
          (:then_1
            (goto _label_2 Reset))))
      (:Released
        (Utilities|FlowControl|Sequence
          (:then_0
            (Utilities|FlowControl|DoOnce false :!label _label_2
              (:Completed
                (Default|CallOnReleasedVK _returnvalue _keyinfo))))
          (:then_1
            (goto _label Reset)))))))

(event EventBeginPlay
  (Variables|Default|SetBaseLocation (Transformation|GetActorLocation)))

(event Collision|EventActorBeginOverlap
  (params (OtherActor :type Actor%20Object%20Reference)))

(event EventTick
  (params (DeltaSeconds :type Float%20%28single-precision%29)))

(fn ConstructionScript)