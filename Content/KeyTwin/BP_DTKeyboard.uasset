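; Virtual keyboard actor that forwards physical key presses and releases to every BP_DTKey in the level.
; On BeginPlay it collects CineCameraActors tagged TargetCamera, views the last one, and binds to each key's press and release dispatchers, unbinding on EndPlay.
; Press events spawn a pooled Niagara burst at the key and play a click sound.
; Release events switch the player's view to the next camera, wrapping around the list.
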(event Custom|OnPressedVK_Event
  (params (KeyLocation :type Vector) (KeyValue :type Key%20Structure :default "None"))
  (Niagara|SpawnSystematLocation "/Game/KeyTwin/NS_Burst.NS_Burst" KeyLocation "0, 0, 0" "1.000000,1.000000,1.000000" true true "AutoRelease")
  (Audio|PlaySound2D "/Game/KeyTwin/btn0.btn0" 1.0 1.0 0.0 0 0))

(event Custom|OnReleasedVK_Event
  (params (KeyLocation :type Vector) (KeyValue :type Key%20Structure :default "None"))
  (CallFunction|ChangeTargetCamera (Variables|Default|GetCameraIndex)))

(event Custom|BindEvent
  ;[0.15 0.15 0.15 0.5] DTKey Press/Release Bind/Unbind
  (for _array_element (Variables|Default|GetKeyList)
    (EventDispatchers|AssignOnPressedVK _array_element (EventDispatchers|CreateEvent :!event Custom|OnPressedVK_Event))
    (EventDispatchers|AssignOnReleasedVK _array_element (EventDispatchers|CreateEvent :!event Custom|OnReleasedVK_Event))))

(event Custom|UnbindEvent
  (bind _keylist (Variables|Default|GetKeyList))
  ;[0.15 0.15 0.15 0.5] DTKey Press/Release Bind/Unbind
  (EventDispatchers|UnbindEventfromOnPressedVK _keylist (EventDispatchers|CreateEvent :!event Custom|OnPressedVK_Event))
  (EventDispatchers|UnbindEventfromOnReleasedVK _keylist (EventDispatchers|CreateEvent :!event Custom|OnReleasedVK_Event)))

(event Custom|ChangeTargetCamera
  (params (SelectedIndex :type Integer))
  (bind _returnvalue (+ SelectedIndex 1))
  (if (!= SelectedIndex -1)
    (Variables|Default|SetCameraIndex (Math|Integer|SelectInt 0 _returnvalue (> _returnvalue (Utilities|Array|LastIndex (Variables|Default|GetCameraList)))))
    (Game|Player|SetViewTargetwithBlend (Game|GetPlayerController 0) (Utilities|Array|Get(acopy) (Variables|Default|GetCameraList) SelectedIndex) 0.0 "VTBlend_Linear" 0.0 false)))

(event EventBeginPlay
  (Utilities|FlowControl|Sequence
    (:then_0
      (bind _outactors (Actor|GetAllActorsOfClasswithTag "/Script/CinematicCamera.CineCameraActor" "TargetCamera"))
      (bind _output_get (Variables|Default|SetCameraList _outactors))
      (CallFunction|ChangeTargetCamera (Utilities|Array|LastIndex _output_get)))
    (:then_1
      (bind _outactors_2 (Actor|GetAllActorsOfClass "/Game/KeyTwin/BP_DTKey.BP_DTKey_C"))
      (Variables|Default|SetKeyList _outactors_2)
      (CallFunction|BindEvent))))

(event EventEndPlay
  (params (EndPlayReason :type EEndPlayReason%20Enum :default "Destroyed"))
  (Utilities|FlowControl|Sequence
    (:then_0
      (CallFunction|UnbindEvent))
    (:then_1
      (|CallParentFunction EndPlayReason))))

(event Input|KeyboardEvents|AnyKey
  (params (Key :type Key%20Structure :default "None"))
  (:Pressed
    (Development|PrintString "[Input Stack] Receive Actor Input")
    (for _array_element (Variables|Default|GetKeyList)
      (Default|PressKey _array_element Key)))
  (:Released
    (for _array_element_2 (Variables|Default|GetKeyList)
      (Default|ReleaseKey _array_element_2 Key))))

(fn ConstructionScript)